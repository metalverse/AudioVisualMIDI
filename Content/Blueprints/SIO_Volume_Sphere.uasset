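; Sound-interactive sphere actor that grows with microphone volume and explodes with an emitter and sound before destroying itself once volume exceeds a threshold.
; Each tick it swivels the mesh around two cone-tilted axes set in the construction script and bobs it vertically by summing three sine waves with separate periods.
; The pitch-range check in NewSoundInteraction has no effect, and the sound-recorded delegate binding never runs.
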(event Custom|NewSoundInteraction
  (params (currentPitchId :type Integer))
  (if (and (>= currentPitchId (Variables|Default|GetMinRangePitchId)) (<= currentPitchId (Variables|Default|GetMaxRangePitchId)))
    _))

(event EventBeginPlay
  (|CallParentFunction))

(event Collision|EventActorBeginOverlap
  (params (OtherActor :type Actor%20Object%20Reference)))

(event EventTick
  (params (DeltaSeconds :type Float%20%28single-precision%29))
  (bind _returnvalue (Transformation|GetActorLocation))
  (bind _returnvalue_2 (Utilities|Time|GetWorldDeltaSeconds))
  (bind _returnvalue_3 (* DeltaSeconds 3.6e+02))
  (bind _microphoneinput (Variables|Default|GetMicrophoneInput))
  (bind _meshlocation (Variables|Bobbing|GetMeshLocation))
  (bind _volumetosizemultiplier (Variables|VolumeAdapter|GetVolumeToSizeMultiplier))
  (bind _minimalsize (Variables|VolumeAdapter|GetMinimalSize))
  (bind _returnvalue_4 (* _returnvalue_2 3.6e+02))
  (bind _returnvalue_5 (+ _returnvalue _meshlocation))
  (bind _volume (Variables|/Script/Midi_Project.MicrophoneInput|Getvolume _microphoneinput))
  (bind _returnvalue_6 (* _volume _volumetosizemultiplier))
  (bind _returnvalue_7 (+ _returnvalue_6 _minimalsize))
  (Variables|Swivel|SetCurrentSwivelX (Math|Float|%(Float) (+ (/ _returnvalue_3 (Variables|Swivel|GetSwivelPeriodX)) (Variables|Swivel|GetCurrentSwivelX)) 3.6e+02))
  (Variables|Swivel|SetCurrentSwivelY (Math|Float|%(Float) (+ (/ _returnvalue_3 (Variables|Swivel|GetSwivelPeriodY)) (Variables|Swivel|GetCurrentSwivelY)) 3.6e+02))
  (Transformation|SetRelativeRotation (Variables|Default|GetMainMesh) (Math|Rotator|MakeRotfromXY (Math|Vector|RotateVectorAroundAxis (Variables|Swivel|GetSwivelAxisX) (Variables|Swivel|GetCurrentSwivelX) "1.000000, 0, 0") (Math|Vector|RotateVectorAroundAxis (Variables|Swivel|GetSwivelAxisY) (Variables|Swivel|GetCurrentSwivelY) "0,1.000000, 0")) false false)
  (Utilities|FlowControl|Sequence
    (:then_0
      (Variables|Bobbing|SetBobbingCycle1 (Math|Float|%(Float) (+ (Variables|Bobbing|GetBobbingCycle1) (/ _returnvalue_4 (Variables|Bobbing|GetBobbingPeriod1))) 3.6e+02)))
    (:then_1
      (Variables|Bobbing|SetBobbingCycle2 (Math|Float|%(Float) (+ (Variables|Bobbing|GetBobbingCycle2) (/ _returnvalue_4 (Variables|Bobbing|GetBobbingPeriod2))) 3.6e+02)))
    (:then_2
      (Variables|Bobbing|SetBobbingCycle3 (Math|Float|%(Float) (+ (Variables|Bobbing|GetBobbingCycle3) (/ _returnvalue_4 (Variables|Bobbing|GetBobbingPeriod3))) 3.6e+02)))
    (:then_3
      (Transformation|SetRelativeLocation (Variables|Default|GetMainMesh) (+ (Variables|Bobbing|GetMeshLocation) (Math|Vector|MakeVector 0.0 0.0 (+ (* (Variables|Bobbing|GetBobbingAmplitude1) (Math|Trig|Sin(Degrees) (Variables|Bobbing|GetBobbingCycle1))) (* (Variables|Bobbing|GetBobbingAmplitude2) (Math|Trig|Sin(Degrees) (Variables|Bobbing|GetBobbingCycle2))) (* (Variables|Bobbing|GetBobbingAmplitude3) (Math|Trig|Sin(Degrees) (Variables|Bobbing|GetBobbingCycle3)))))) false false)
      (Transformation|SetActorScale3D (Math|Vector|MakeVector _returnvalue_7 _returnvalue_7 _returnvalue_7))
      (if (> _volume (Variables|VolumeAdapter|GetDestroyVolume))
        (Effects|SpawnEmitteratLocation "/Game/Effects/Great_Explosion.Great_Explosion" _returnvalue_5)
        (Audio|SpawnSoundatLocation "/Game/FirstPerson/Audio/FirstPersonTemplateWeaponFire02.FirstPersonTemplateWeaponFire02" _returnvalue_5)
        (Actor|DestroyActor)))))

(fn ConstructionScript
  (|CallParentFunction)
  (Variables|Swivel|SetSwivelAxisX (Math|Vector|RotateVectorAroundAxis "1.000000,0.000000, 0" (Variables|Swivel|GetSwivelConeX) "0, 0,1.000000"))
  (Variables|Swivel|SetSwivelAxisY (Math|Vector|RotateVectorAroundAxis "0,1.000000, 0" (Variables|Swivel|GetSwivelConeY) "0, 0,1.000000")))