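; MIDI-driven percussion visualizer that builds a set of antenna meshes at supplied positions and animates them from note events.
; High-hat note-ons spawn an electricity beam between neighboring antennas, chosen by note index, with a timer or other event type clearing all arcs.
; Otherwise, an upcoming drum note spawns note-colored light discs above every antenna, passing each the time difference and antenna position to visualize the sound.
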(event Custom|Construct%20Antenas
  (params (AntenaPositions :type Array%20of%20Vectors))
  ;[1 1 1] Construct Antenas
  (bind _output_get (Variables|Default|SetAntenaPositions AntenaPositions))
  (for _array_element _output_get
    (bind _returnvalue (AddComponent|AddStaticMeshComponent false (Math|Transform|MakeTransform _array_element "0, 0, 0" "1,1,2.000000")))
    (Utilities|Array|AddUnique (Variables|Default|GetAntenas) _returnvalue)
    (Components|StaticMesh|SetStaticMesh _returnvalue "/Game/Assets/Scene/Antena.Antena")))

(event EventBeginPlay)

(event Collision|EventActorBeginOverlap
  (params (OtherActor :type Actor%20Object%20Reference)))

(event EventMidiInteraction
  (params (CurrentNote :type Integer) (NextNote :type Integer) (TimeDifference :type Integer) (EventType :type Integer))
  (bind _high_hats (Variables|Default|GetHigh-Hats))
  (if (Utilities|Array|ContainsItem _high_hats CurrentNote)
    (if (== EventType (Variables|Default|GetMidiNoteOn))
      (CallFunction|SpawnEmitter (Math|Integer|%(Integer) (Utilities|Array|FindItem _high_hats CurrentNote) (Utilities|Array|Length (Variables|Default|GetEmitters))))
      (Utilities|Time|SetTimerbyFunctionName 0 "DestroyEmitters" (/ 1.0 (/ (Math|Conversions|ToFloat(Integer) TimeDifference) 1e+03)))
      (else
        (CallFunction|DestroyEmitters)))
    (elif (Utilities|Array|ContainsItem (Variables|Default|GetDrums) NextNote)
      (bind _notecolor (CallFunction|GetColorbyNoteId NextNote))
      (for _array_element (Variables|Default|GetAntenas)
        (bind _returnvalue (Game|SpawnActorfromClass "/Game/Blueprints/PercussionLightDisc.PercussionLightDisc_C" (Math|Transform|MakeTransform (Math|Vector|MakeVector (.x (Transformation|GetWorldLocation _array_element)) (.y (Transformation|GetWorldLocation _array_element)) (+ (.z (Transformation|GetWorldLocation _array_element)) (Variables|Default|GetAntenaHeight))) "0, 0, 0" "1,1,1") "Undefined" 0 _notecolor (Math|Vector|MakeVector (.x (Transformation|GetWorldLocation _array_element)) (.y (Transformation|GetWorldLocation _array_element)) (+ (.z (Transformation|GetWorldLocation _array_element)) (Variables|Default|GetAntenaHeight)))))
        (Default|VisualizeSound _returnvalue TimeDifference (Transformation|GetWorldLocation _array_element))))))

(event EventTick
  (params (DeltaSeconds :type Float%20%28single-precision%29)))

(fn ConstructionScript
  (Variables|Default|SetEmitters (Utilities|Array|MakeArray (Variables|Default|GetEmitter12) (Variables|Default|GetEmitter23) (Variables|Default|GetEmitter34) (Variables|Default|GetEmitter45) (Variables|Default|GetEmitter56) (Variables|Default|GetEmitter61))))

(fn SpawnEmitter
  (params (Index :type Integer))
  (bind _returnvalue (+ Index 1))
  (bind _emitters (Variables|Default|GetEmitters))
  (bind _antenas (Variables|Default|GetAntenas))
  (bind _antenas_2 (Variables|Default|GetAntenas))
  (bind _item (Utilities|Array|Get(acopy) _emitters Index))
  (bind _returnvalue_2 (Utilities|Array|Length _antenas_2))
  (bind _item_2 (Utilities|Array|Get(acopy) _antenas Index))
  (bind _returnvalue_3 (Math|Integer|%(Integer) _returnvalue _returnvalue_2))
  (bind _returnvalue_4 (Transformation|GetWorldLocation _item_2))
  (bind _item_3 (Utilities|Array|Get(acopy) _antenas_2 _returnvalue_3))
  (bind _returnvalue_5 (Transformation|GetWorldLocation _item_3))
  (Utilities|IsValid _item
    (:Is%20Valid
      (Actor|DestroyActor _item))
    (:Is%20Not%20Valid
      _))
  (bind _returnvalue_6 (Game|SpawnActorfromClass "/Game/ElectricityArc_BP.ElectricityArc_BP_C" (Math|Transform|MakeTransform (Math|Vector|MakeVector (.x _returnvalue_4) (.y _returnvalue_4) (+ (.z _returnvalue_4) (Variables|Default|GetAntenaHeight))) "0.000000, 0, 0" "1.000000,1,1") "AlwaysSpawn" 0 0))
  (Class|ParticleSystemComponent|SetBeamTargetPoint (Variables|/Game/ElectricityArc_BP.ElectricityArc_BP_C|GetEmitter _returnvalue_6) 0 (Math|Vector|MakeVector (.x _returnvalue_5) (.y _returnvalue_5) (+ (.z _returnvalue_5) (Variables|Default|GetAntenaHeight))))
  (Utilities|Array|SetArrayElem (Variables|Default|GetEmitters) Index _returnvalue_6))

(fn DestroyEmitters
  (for _array_element (Variables|Default|GetEmitters)
    (Utilities|IsValid _array_element
      (:Is%20Valid
        (Actor|DestroyActor _array_element)))))