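; PercussionLightDisc is an actor that visualizes a sound as a colored disc flying to a target and bursting.
; The construction script creates a dynamic material, which BeginPlay tints with ActiveColor.
; VisualizeSound runs a timeline that lerps the actor from StartPosition to TargetPosition, then spawns a small explosion and destroys it.
; TimeDifference is stored, but the play-rate scaling that uses it is disconnected, so travel time ignores it.
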(event Custom|VisualizeSound
  (params (TimeDifference :type Integer) (TargetPosition :type Vector))
  (Variables|Default|SetTargetPosition TargetPosition)
  (bind _output_get (Variables|Default|SetTimeDifference TimeDifference))
  (bind _alpha (Timeline|Timeline_0 PlayFromStart)
    (:Update
      (Transformation|SetActorLocation (Math|Vector|Lerp(Vector) (Variables|Default|GetStartPosition) (Variables|Default|GetTargetPosition) _alpha) false false))
    (:Finished
      (Effects|SpawnEmitteratLocation "/Game/Effects/Small_Explosion.Small_Explosion" (Variables|Default|GetTargetPosition))
      (Actor|DestroyActor))))

(event EventBeginPlay
  (Rendering|Material|SetVectorParameterValue (Variables|Default|GetMaterial) "Color" (Variables|Default|GetActiveColor) :!class /Script/Engine.MaterialInstanceDynamic))

(event Collision|EventActorBeginOverlap
  (params (OtherActor :type Actor%20Object%20Reference)))

(event EventTick
  (params (DeltaSeconds :type Float%20%28single-precision%29)))

(fn ConstructionScript
  (bind _returnvalue (Rendering|Material|CreateDynamicMaterialInstance (Variables|Default|GetStaticMesh) 0 "/Game/Materials/LevitatingSphere/LevitatingSphere_Inactive.LevitatingSphere_Inactive" :!class /Script/Engine.PrimitiveComponent))
  (Variables|Default|SetMaterial _returnvalue))