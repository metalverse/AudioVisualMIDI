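; BP_Sound_Interactive_Object is a skeletal actor, apparently a base, for objects that react to MIDI notes and sound input.
; It declares empty events for MIDI interaction, note ID and onset input, and widget removal.
; GetColorByNoteId wraps note IDs modulo 12 into ToneColors, giving each pitch class one color across octaves.
; CalculateProgress returns the received value over the value needed for interaction, clamped between zero and one.
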(event Custom|RemoveWidget)

(event Custom|MidiInteraction
  (params (CurrentNote :type Integer) (NextNote :type Integer) (TimeDifference :type Integer) (EventType :type Integer)))

(event Custom|HandleInputOnset)

(event Custom|HandleInputNoteId
  (params (NoteId :type Integer) (Value :type Integer)))

(event EventBeginPlay)

(event Collision|EventActorBeginOverlap
  (params (OtherActor :type Actor%20Object%20Reference)))

(event EventTick
  (params (DeltaSeconds :type Float%20%28single-precision%29)))

(fn ConstructionScript)

(fn GetColorbyNoteId
  (params (NoteId :type Integer))
  (return (Utilities|Array|Get(acopy) (Variables|Default|GetToneColors) (Math|Integer|%(Integer) NoteId 12))))

(fn CalculateProgress
  (return (Math|Float|Clamp(Float) (/ (Math|Conversions|ToFloat(Integer) (Variables|Default|GetReceivedValue)) (Math|Conversions|ToFloat(Integer) (Variables|Default|GetValueNeededForInteraction))))))