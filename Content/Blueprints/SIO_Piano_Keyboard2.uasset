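; Sound-interactive piano keyboard actor that lights up a bar for each pitch detected by its PitchTracker.
; On BeginPlay it builds a centred row of tall thin meshes with dynamic materials and a palette of random colours.
; Each recorded pitch within range blacks out the previous bar and tints the bar indexed by pitch ID with a random palette colour.
; Statue spawning and note-name printing remain as unconnected nodes.
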(event Custom|NewSoundInteraction
  (params (currentPitchId :type Integer))
  (bind _visualcubescolors (Variables|Default|GetVisualCubesColors))
  (if (and (>= currentPitchId (Variables|Default|GetMinRangePitchId)) (<= currentPitchId (Variables|Default|GetMaxRangePitchId)))
    (Utilities|FlowControl|Sequence
      (:then_0
        (Rendering|Material|SetVectorParameterValue (Utilities|Array|Get(acopy) (Variables|Default|GetVisualCubes) (Variables|Default|GetLastNoteIndex)) "Color" (Math|Color|SelectColor :B "(R=0.000000,G=0.000000,B=0.000000,A=1.000000)" :bPickA true) :!class /Script/Engine.MaterialInstanceDynamic))
      (:then_1
        (bind _output_get (Variables|Default|SetCurrentPitchId currentPitchId))
        (Variables|Default|SetLastNoteIndex _output_get)
        (Rendering|Material|SetVectorParameterValue (Utilities|Array|Get(acopy) (Variables|Default|GetVisualCubes) _output_get) "Color" (Math|Color|SelectColor (Utilities|Array|Get(acopy) _visualcubescolors (Math|Random|RandomIntegerinRange 0 (- (Utilities|Array|Length _visualcubescolors) 1))) "(R=0.000000,G=0.000000,B=0.000000,A=1.000000)" true) :!class /Script/Engine.MaterialInstanceDynamic)))))

(event EventBeginPlay
  (|CallParentFunction)
  (EventDispatchers|BindEventtoOnSoundRecordedDelegate (Variables|Default|GetPitchTracker) (delegate Custom|NewSoundInteraction))
  ;[1 1 1] Create Visual Cubes
  (for _index (range 0 115)
    (bind _returnvalue (AddComponent|AddStaticMeshComponent false (Math|Transform|MakeTransform (Math|Vector|MakeVector 0.0 (- (* _index 1e+01) 5.8e+02) 0.0) "0, 0, 0" "0.050000,0.050000,1.500000")))
    (Collision|SetCollisionObjectType _returnvalue "ECC_WorldStatic")
    (bind _returnvalue_2 (Rendering|Material|CreateDynamicMaterialInstance _returnvalue 0 "/Game/Materials/MatTest.MatTest" :!class /Script/Engine.PrimitiveComponent))
    (Utilities|Array|Add (Variables|Default|GetVisualCubes) _returnvalue_2))
  (for _index_2 (range 0 20)
    (Utilities|Array|Add (Variables|Default|GetVisualCubesColors) (Utilities|Struct|MakeLinearColor (Math|Random|RandomFloat) (Math|Random|RandomFloat) (Math|Random|RandomFloat) 1.0))))

(event Collision|EventActorBeginOverlap
  (params (OtherActor :type Actor%20Object%20Reference)))

(event EventTick
  (params (DeltaSeconds :type Float%20%28single-precision%29)))

(fn ConstructionScript)