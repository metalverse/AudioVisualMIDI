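; Microphone input Blueprint that turns detected pitch, silence, onsets and tempo into game sound events.
; BeginPlay initializes Vamp audio-analysis plugins with GameInstance onset settings and finds the BP_MidiManager.
; Outside calibration, Tick forwards tempo changes to MIDI and the HUD, and accepts a buffered note only when it holds a majority of occurrences.
; Sound on/modify/off and volume events follow from note, silence and onset states, alongside matching detection callbacks.
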(event EventBeginPlay
  ;[1 1 1] Begin Play
  (CallFunction|InitVampPluginswithParams)
  (bind _outactors (Actor|GetAllActorsOfClass "/Game/Blueprints/BP_MidiManager.BP_MidiManager_C"))
  (Utilities|IsValid (Utilities|Array|Get(acopy) _outactors)
    (:Is%20Valid
      (Variables|Default|SetMidiComponent (Utilities|Array|Get(acopy) _outactors)))
    (:Is%20Not%20Valid
      (Development|PrintString "MicrophoneInput: Visual Player not valid!" true true "(R=1.000000,G=0.000000,B=0.000000,A=1.000000)" 8.0))))

(event Collision|EventActorBeginOverlap
  (params (OtherActor :type Actor%20Object%20Reference)))

(event EventTick
  (params (DeltaSeconds :type Float%20%28single-precision%29))
  (bind _soundeventmodes (Variables|Default|GetSoundEventModes))
  (if (not (Variables|Default|GetisInCallibrationMode))
    (if (Variables|Default|GetprepareForTempoChange)
      (Class|MidiComponent|PrepareforTempoChange (Variables|/Game/Midi/Player/BP_Asset_Player.BP_Asset_Player_C|GetMidi (Variables|Default|GetMidiComponent))))
    (if (Variables|Default|GetnewTempoTracked)
      (Default|ChangeMIDITempo (Variables|Default|GetMidiComponent) (Variables|Default|GettrackedTempoInBpm))
      (CallFunction|NotifyWidgetAboutTempoChange))
    (bind (_noteavailable _noteid _value) (CallFunction|CheckNotesBuffer))
    (if _noteavailable
      (Variables|Default|SetCurrentMidiNote _noteid)
      (Variables|Default|SetCurrentMidiNoteOccurrences _value)
      (if (Variables|Default|GetWasSilence)
        (Variables|Default|SetWasSilence false)
        (Development|PrintString "Sound!")
        (Class|SoundComponent|CallSoundEvent (Variables|Default|GetSound) (.soundon (Variables|Default|GetSoundEventModes)) (Variables|Default|GetCurrentMidiNoteOccurrences) (Variables|Default|GetCurrentMidiNote) (Variables|Default|GetvolumedB))
        (else
          (Class|SoundComponent|CallSoundEvent (Variables|Default|GetSound) (.soundmodify (Variables|Default|GetSoundEventModes)) (Variables|Default|GetCurrentMidiNoteOccurrences) (Variables|Default|GetCurrentMidiNote) (Variables|Default|GetvolumedB))))
      (Default|CallOnSoundDetected (Variables|Default|GetCurrentMidiNote) (Variables|Default|GetCurrentMidiNoteOccurrences))
      (Variables|Default|SetIsSoundOn true)
      (CallFunction|ClearBuffers)
      (elif (Variables|Default|GetisSilence)
        (if (not (Variables|Default|GetWasSilence))
          (Variables|Default|SetWasSilence true)
          (Development|PrintString "Silence")
          (Class|SoundComponent|CallSoundEvent (Variables|Default|GetSound) (.soundoff _soundeventmodes) 0 0 0.0)
          (Variables|Default|SetIsSoundOn false)
          (Default|CallOnSilenceDetected))
        (elif (not (Variables|Default|GetisWaitingForData))
          (CallFunction|ClearBuffers)
          (if (not (Variables|Default|GetIsSoundOn))
            (if (Variables|Default|GetisOnsetDetected)
              (Class|SoundComponent|CallSoundEvent (Variables|Default|GetSound) (.volumeevent _soundeventmodes) 0 0 (Variables|Default|GetvolumedB))
              (Default|CallOnOnsetDetected)
              (Development|PrintString "Onset!" true true "(R=0.000000,G=0.660000,B=1.000000,A=1.000000)" 8.0))))))))

(fn ConstructionScript)

(fn CheckNotesBuffer
  (for (_array_element _array_index) (Variables|Default|GetbufferedMidiNotesOccurences)
    (LocalVariables|SetOccurencesSum (+ (LocalVariables|GetOccurencesSum) _array_element))
    (if (> _array_element (LocalVariables|GetMaxOccurences))
      (LocalVariables|SetMaxOccurences _array_element)
      (LocalVariables|SetMaxOccurencesNoteIndex _array_index)))
  (if (> (LocalVariables|GetMaxOccurences) (/ (LocalVariables|GetOccurencesSum) 2))
    (if (!= (Utilities|Array|Get(acopy) (Variables|Default|GetbufferedMidiNotes) (LocalVariables|GetMaxOccurencesNoteIndex)) -1)
      (return true (Utilities|Array|Get(acopy) (Variables|Default|GetbufferedMidiNotes) (LocalVariables|GetMaxOccurencesNoteIndex)) (LocalVariables|GetMaxOccurences))
      (else
        _)))
  (return false 0 0))

(fn ClearBuffers
  (Utilities|Array|Clear (Variables|Default|GetbufferedMidiNotes))
  (Utilities|Array|Clear (Variables|Default|GetbufferedMidiNotesOccurences)))

(fn GetNoiseLevel
  (return (/ 0.0 (Math|Conversions|ToFloat(Integer) 0))))

(fn NotifyWidgetAboutTempoChange
  (bind _foundwidgets (Widget|GetAllWidgetsOfClass "/Game/HUD/UserHUD.UserHUD_C" true))
  (Utilities|IsValid (Utilities|Array|Get(acopy) _foundwidgets)
    (:Is%20Valid
      (Default|HandleTempoMode (Utilities|Array|Get(acopy) _foundwidgets))
      (Development|PrintString "AAAAAAAAAAAAAAAAA"))))

(fn InitVampPluginswithParams
  (bind _asmy_game_instance (Utilities|Casting|CastToMyGameInstance (Game|GetGameInstance)))
  (Variables|Default|SetonsetParamThreshold (Variables|/Game/GameInstances/MyGameInstance.MyGameInstance_C|GetOnsetDetectorThreshold _asmy_game_instance))
  (Variables|Default|SetonsetParamSensitivity (Variables|/Game/GameInstances/MyGameInstance.MyGameInstance_C|GetOnsetDetectorSensitivity _asmy_game_instance))
  (Class|MicrophoneInput|InitVampPlugins))