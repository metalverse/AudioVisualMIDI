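; Hex floor tile actor that animates itself once, moving vertically and then opening, on a fixed delay after BeginPlay.
; A first timeline offsets the root along local Z by ZOffset, applying per-update alpha deltas as relative movement.
; When it finishes, a second timeline drives the skeletal mesh's Opened_Tile morph target.
; Despite the Interactive name, overlap and Tick events are unused.
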(event EventBeginPlay
  (Utilities|FlowControl|Delay 5.0)
  (bind _alpha (Timeline|Timeline_0 PlayFromStart)
    (:Update
      (Transformation|AddLocalOffset (Variables|Default|GetDefaultSceneRoot) (Math|Vector|MakeVector 0.0 0.0 (* (- _alpha (Variables|Default|GetLastAlpha)) (Variables|Default|GetZOffset))) false false)
      (Variables|Default|SetLastAlpha _alpha))
    (:Finished
      (bind _alpha_2 (Timeline|Timeline_1 PlayFromStart)
        (:Update
          (Components|SkeletalMesh|SetMorphTarget (Variables|Default|GetSkeletalMesh) "Opened_Tile" _alpha_2 true))))))

(event Collision|EventActorBeginOverlap
  (params (OtherActor :type Actor%20Object%20Reference)))

(event EventTick
  (params (DeltaSeconds :type Float%20%28single-precision%29)))

(fn ConstructionScript)