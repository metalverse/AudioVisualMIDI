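; Floating scene object that swivels, bobs and reacts to the beat with color.
; On BeatComponent beats, a chance roll restarts a timeline that blends the dynamic material from a randomized base color toward dark teal.
; Tick throttles motion by accumulated time, rotating around cone-offset axes from construction and summing three sine waves for vertical bobbing.
; The sound interaction event is empty and the Tracker recording binding is unconnected.
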(event Custom|TempoEvent
  (params (Mode :type Integer) (Value :type Integer))
  (if (>= (Variables|Default|GetChanceForAction) (Math|Random|RandomIntegerinRange 0 100))
    (bind _alpha (Timeline|ColorBlendTimeline PlayFromStart)
      (:Update
        (Rendering|Material|SetVectorParameterValue (Variables|Default|GetMaterial) "Color" (Math|Color|Lerp(LinearColor) (Variables|Default|GetColor) "(R=0.000000,G=0.025483,B=0.035000,A=1.000000)" _alpha) :!class /Script/Engine.MaterialInstanceDynamic)))))

(event Custom|NewSoundInteraction
  (params (currentPitchId :type Integer)))

(event EventBeginPlay
  (|CallParentFunction)
  (bind _returnvalue (Rendering|Material|CreateDynamicMaterialInstance (Variables|Default|GetMainMesh) 0 "/Game/Midi/Other/MatTest.MatTest" :!class /Script/Engine.PrimitiveComponent))
  (Variables|Default|SetMaterial _returnvalue)
  (Variables|Default|SetColor (Utilities|Struct|MakeLinearColor (Math|Random|RandomFloatinRange 0.18 0.25) (Math|Random|RandomFloatinRange 0.7 0.85) (Math|Random|RandomFloatinRange 0.68 0.73) 1.0))
  (EventDispatchers|BindEventtoOnEventBeat (Variables|Default|GetBeatComponent) (delegate Custom|TempoEvent)))

(event Collision|EventActorBeginOverlap
  (params (OtherActor :type Actor%20Object%20Reference)))

(event EventTick
  (params (DeltaSeconds :type Float%20%28single-precision%29))
  (bind _returnvalue (Utilities|Time|GetWorldDeltaSeconds))
  (bind _returnvalue_2 (* _returnvalue 3.6e+02))
  (bind _output_get (Variables|Default|SetdeltaSeconds (+ (Variables|Default|GetdeltaSeconds) DeltaSeconds)))
  (if (> _output_get 0.05)
    (Variables|Swivel|SetCurrentSwivelX (Math|Float|%(Float) (+ (/ (* _output_get 3.6e+02) (Variables|Swivel|GetSwivelPeriodX)) (Variables|Swivel|GetCurrentSwivelX)) 3.6e+02))
    (Variables|Swivel|SetCurrentSwivelY (Math|Float|%(Float) (+ (/ (* _output_get 3.6e+02) (Variables|Swivel|GetSwivelPeriodY)) (Variables|Swivel|GetCurrentSwivelY)) 3.6e+02))
    (Transformation|SetRelativeRotation (Variables|Default|GetScene) (Math|Rotator|MakeRotfromXY (Math|Vector|RotateVectorAroundAxis (Variables|Swivel|GetSwivelAxisX) (Variables|Swivel|GetCurrentSwivelX) "1.000000, 0, 0") (Math|Vector|RotateVectorAroundAxis (Variables|Swivel|GetSwivelAxisY) (Variables|Swivel|GetCurrentSwivelY) "0.000000,1.000000, 0")) false false)
    (Utilities|FlowControl|Sequence
      (:then_0
        (Variables|Bobbing|SetBobbingCycle1 (Math|Float|%(Float) (+ (Variables|Bobbing|GetBobbingCycle1) (/ _returnvalue_2 (Variables|Bobbing|GetBobbingPeriod1))) 3.6e+02)))
      (:then_1
        (Variables|Bobbing|SetBobbingCycle2 (Math|Float|%(Float) (+ (Variables|Bobbing|GetBobbingCycle2) (/ _returnvalue_2 (Variables|Bobbing|GetBobbingPeriod2))) 3.6e+02)))
      (:then_2
        (Variables|Bobbing|SetBobbingCycle3 (Math|Float|%(Float) (+ (Variables|Bobbing|GetBobbingCycle3) (/ _returnvalue_2 (Variables|Bobbing|GetBobbingPeriod3))) 3.6e+02)))
      (:then_3
        (Transformation|SetRelativeLocation (Variables|Default|GetScene) (+ (Variables|Bobbing|GetActorLocation) (Math|Vector|MakeVector 0.0 0.0 (+ (* (Variables|Bobbing|GetBobbingAmplitude1) (Math|Trig|Sin(Degrees) (Variables|Bobbing|GetBobbingCycle1))) (* (Variables|Bobbing|GetBobbingAmplitude2) (Math|Trig|Sin(Degrees) (Variables|Bobbing|GetBobbingCycle2))) (* (Variables|Bobbing|GetBobbingAmplitude3) (Math|Trig|Sin(Degrees) (Variables|Bobbing|GetBobbingCycle3)))))) false false)
        (Variables|Default|SetdeltaSeconds 0.0)))))

(fn ConstructionScript
  (|CallParentFunction)
  (Variables|Swivel|SetSwivelAxisX (Math|Vector|RotateVectorAroundAxis "1.000000,0.000000, 0" (Variables|Swivel|GetSwivelConeX) "0, 0,1.000000"))
  (Variables|Swivel|SetSwivelAxisY (Math|Vector|RotateVectorAroundAxis "0,1.000000, 0" (Variables|Swivel|GetSwivelConeY) "0, 0,1.000000"))
  (Variables|VolumeAdapter|SetVolumeToSizeMultiplier (/ (- (Variables|VolumeAdapter|GetMaximalSize) (Variables|VolumeAdapter|GetMinimalSize)) (Variables|VolumeAdapter|GetDestroyVolume))))