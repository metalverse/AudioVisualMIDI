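; Interactive statue tied to one MIDI instrument channel, which reacts to song notes and player sound input by pulsing its material color.
; MIDI events drive a timeline fading from note color to idle, timed by note spacing.
; In certain modes, detected input notes play on the channel and silence stops them.
; Onset counts trigger channel mixing changes through BP_MidiManager, some also copying the interaction mode to all other statues.
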(event Custom|ChangeMode
  (params (NewStatus :type InstrumentState%20Enum))
  (Variables|Default|SetInteractionMode NewStatus))

(event EventBeginPlay
  (bind _returnvalue (Rendering|Material|CreateDynamicMaterialInstance (Variables|Default|GetStaticMesh) 0 "/Game/Materials/MatTest.MatTest" :!class /Script/Engine.PrimitiveComponent))
  (Variables|Default|SetMaterial _returnvalue)
  (Variables|Default|SetActorLocation (Transformation|GetWorldLocation (Variables|Default|GetStaticMesh)))
  (bind _outactors (Actor|GetAllActorsOfClass "/Game/Blueprints/BP_MidiManager.BP_MidiManager_C"))
  (Utilities|IsValid (Utilities|Array|Get(acopy) _outactors)
    (:Is%20Valid
      (Variables|Default|SetVisual_Midi (Utilities|Array|Get(acopy) _outactors)))))

(event Collision|EventActorBeginOverlap
  (params (OtherActor :type Actor%20Object%20Reference)))

(event EventHandleInputNoteId
  (params (NoteId :type Integer) (Value :type Integer))
  (bind _visual_midi (Variables|Default|GetVisual_Midi))
  ;[1 1 1] Handle Input Note Id
  (if (or (Utilities|Enum|Equal(Enum) (Variables|Default|GetInteractionMode) "NewEnumerator1") (Utilities|Enum|Equal(Enum) (Variables|Default|GetInteractionMode) "NewEnumerator0"))
    (if (!= (- NoteId 12) (Variables|Default|GetCurrentNotePlaying))
      (Default|StopMidiNoteonChannel _visual_midi (Variables|Default|GetInstrumentChannel) (Variables|Default|GetCurrentNotePlaying))
      (bind _output_get (Variables|Default|SetCurrentNotePlaying (- NoteId 12)))
      (Default|PlayMidiNoteonChannel _visual_midi (Variables|Default|GetInstrumentChannel) _output_get)
      (CallFunction|VoiceInteraction _output_get 3500 (Variables|Default|GetMidiNoteOn)))))

(event EventHandleInputOnset
  ;[1 1 1] Handle Input Onset
  (|CallParentFunction)
  (Development|PrintString (Utilities|String|ToString(Integer) (Variables|Default|GetDetectedInteractionOnsets)) true true "(R=1.000000,G=0.879220,B=0.000000,A=1.000000)" 4.0))

(event EventMidiInteraction
  (params (CurrentNote :type Integer) (NextNote :type Integer) (TimeDifference :type Integer) (EventType :type Integer))
  ;[1 1 1] Midi Interaction
  (if (not (Math|Boolean|ORBoolean (Variables|Default|GetIsInInteractiveMode) (not (Utilities|Enum|Equal(Enum) (Variables|Default|GetInteractionMode) "NewEnumerator2")) (Utilities|Enum|Equal(Enum) (Variables|Default|GetInteractionMode) "NewEnumerator3")))
    (Variables|Default|SetCurrentNoteID CurrentNote)
    (Variables|Default|SetCurrentTimeDifference TimeDifference)
    (Variables|Default|SetCurrentEventType EventType)
    (bind _notecolor (CallFunction|GetColorbyNoteId (Variables|Default|GetCurrentNoteID)))
    (Variables|Default|SetActionColor _notecolor)
    (if (== (Variables|Default|GetCurrentEventType) (Variables|Default|GetMidiNoteOn))
      (Components|Timeline|SetPlayRate (Variables|Default|GetSmoothColorLerp) (/ 1.0 (/ (Math|Conversions|ToFloat(Integer) (Variables|Default|GetCurrentTimeDifference)) 1e+03)))
      (bind _alpha (Timeline|SmoothColorLerp PlayFromStart)
        (:Update
          (Variables|Default|SetCurrentAlpha _alpha)
          (Rendering|Material|SetVectorParameterValue (Variables|Default|GetMaterial) "Color" (Math|Color|Lerp(LinearColor) (Variables|Default|GetActionColor) (Variables|Default|GetIdleColor) _alpha) :!class /Script/Engine.MaterialInstanceDynamic))))))

(event EventTick
  (params (DeltaSeconds :type Float%20%28single-precision%29)))

(event EventHandleInputSilence
  ;[1 1 1] Handle Input Silence
  (if (or (Utilities|Enum|Equal(Enum) (Variables|Default|GetInteractionMode) "NewEnumerator1") (Utilities|Enum|Equal(Enum) (Variables|Default|GetInteractionMode) "NewEnumerator0"))
    (Utilities|FlowControl|Sequence
      (:then_0
        ;[1 1 1] Midi Interaction
        (bind _alpha (Timeline|SmoothColorLerp Stop)
          (:Update
            (Variables|Default|SetCurrentAlpha _alpha)
            (Rendering|Material|SetVectorParameterValue (Variables|Default|GetMaterial) "Color" (Math|Color|Lerp(LinearColor) (Variables|Default|GetActionColor) (Variables|Default|GetIdleColor) _alpha) :!class /Script/Engine.MaterialInstanceDynamic))))
      (:then_1
        (Components|Timeline|SetPlayRate (Variables|Default|GetSmoothLerpSilence) 2.0)
        (bind _alpha_2 (Timeline|SmoothLerpSilence PlayFromStart)
          (:Update
            (Rendering|Material|SetVectorParameterValue (Variables|Default|GetMaterial) "Color" (Math|Color|Lerp(LinearColor) (Variables|Default|GetActionColor) (Variables|Default|GetIdleColor) (Math|Float|Lerp (Variables|Default|GetCurrentAlpha) 1.0 _alpha_2)) :!class /Script/Engine.MaterialInstanceDynamic))
          (:Finished
            (Default|StopMidiNoteonChannel (Variables|Default|GetVisual_Midi) (Variables|Default|GetInstrumentChannel) (Variables|Default|GetCurrentNotePlaying))
            (Variables|Default|SetCurrentNotePlaying 0)))))))

(event EventVoiceInteraction
  (params (MidiNote :type Integer) (TimeDifference :type Integer) (EventType :type Integer))
  ;[1 1 1] Midi Interaction
  ;;[1 1 1] Voice Interaction
  (Variables|Default|SetCurrentNoteID MidiNote)
  (Variables|Default|SetCurrentTimeDifference TimeDifference)
  (Variables|Default|SetCurrentEventType EventType)
  (bind _notecolor (CallFunction|GetColorbyNoteId (Variables|Default|GetCurrentNoteID)))
  (Variables|Default|SetActionColor _notecolor)
  (if (== (Variables|Default|GetCurrentEventType) (Variables|Default|GetMidiNoteOn))
    (Components|Timeline|SetPlayRate (Variables|Default|GetSmoothColorLerp) (/ 1.0 (/ (Math|Conversions|ToFloat(Integer) (Variables|Default|GetCurrentTimeDifference)) 1e+03)))
    (bind _alpha (Timeline|SmoothColorLerp PlayFromStart)
      (:Update
        (Variables|Default|SetCurrentAlpha _alpha)
        (Rendering|Material|SetVectorParameterValue (Variables|Default|GetMaterial) "Color" (Math|Color|Lerp(LinearColor) (Variables|Default|GetActionColor) (Variables|Default|GetIdleColor) _alpha) :!class /Script/Engine.MaterialInstanceDynamic)))))

(event EventChooseInteractionMode
  (bind _visual_midi (Variables|Default|GetVisual_Midi))
  ;[1 1 1] Choose Interaction Mode
  (|CallParentFunction)
  (switch int (Variables|Default|GetDetectedInteractionOnsets)
    (:1
      (Default|ExcludeChannelfromFileData (Variables|Default|GetVisual_Midi) (Utilities|Array|MakeArray (Variables|Default|GetInstrumentChannel)) :!label _label)
      (Default|HandleChannelonFirstPlace (Variables|Default|GetVisual_Midi) (Variables|Default|GetInstrumentChannel))
      (CallFunction|NotifyOtherStatues (Variables|Default|GetInteractionMode)))
    (:2
      (goto _label))
    (:3
      (Variables|Default|SetCanInteract false)
      (Utilities|Time|SetTimerbyFunctionName 0 "ReleaseInteraction" 1.0)
      (if (Utilities|Enum|Equal(Enum) (Variables|Default|GetInteractionMode) "NewEnumerator2")
        (Default|IncludeChanneltoFileData _visual_midi (Utilities|Array|MakeArray (Variables|Default|GetInstrumentChannel)))
        (Default|AllChannelsonSameLevel _visual_midi)
        (else
          (Default|ExcludeChannelfromFileData (Variables|Default|GetVisual_Midi) (Utilities|Array|MakeArray (Variables|Default|GetInstrumentChannel))))))))

(event EventHandleOnsetChangeInteraction
  (bind _visual_midi (Variables|Default|GetVisual_Midi))
  ;[1 1 1] Handle Onset Change Interaction
  (|CallParentFunction)
  (switch int (Variables|Default|GetDetectedInteractionOnsets)
    (:1
      (if (Utilities|Enum|Equal(Enum) (Variables|Default|GetInteractionMode) "NewEnumerator1")
        (CallFunction|SetInstrumentbyLastNote)))
    (:2
      (Variables|Default|SetCanInteract false)
      (Utilities|Time|SetTimerbyFunctionName 0 "ReleaseInteraction" 1.0)
      (Default|IncludeChanneltoFileData _visual_midi (Utilities|Array|MakeArray (Variables|Default|GetInstrumentChannel)))
      (Default|AllChannelsonSameLevel _visual_midi)
      (CallFunction|NotifyOtherStatues (Variables|Default|GetInteractionMode)))))

(fn ConstructionScript)

(fn NotifyOtherStatues
  (params (NewState :type InstrumentState%20Enum))
  (bind _outactors (Actor|GetAllActorsOfClass "SIO_Statue_BP_C"))
  (for _array_element _outactors
    (if (!= _array_element self)
      (CallFunction|ChangeMode _array_element NewState))))