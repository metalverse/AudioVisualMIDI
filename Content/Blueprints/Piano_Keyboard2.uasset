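; Piano keyboard visualizer actor that lights up bars according to the pitch heard through microphone input.
; On BeginPlay it finds BP_MicrophoneInput_Plus, binds to its pitch tracker's sound-recorded delegate, and builds a row of thin bars with dynamic materials plus a random color palette.
; For in-range pitch events, it blacks out the last lit bar and colors the bar indexed by the tracker's current note with a random palette color.
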(event Custom|NewSoundInteraction
  (params (currentPitchId :type Integer))
  (bind _visualcubescolors (Variables|Default|GetVisualCubesColors))
  (bind _pitchtracker (Variables|Default|GetPitchTracker))
  (bind _currentnote (Variables|/Script/Midi_Project.SimplePitchTracker|GetcurrentNote _pitchtracker))
  (Development|PrintString (Utilities|String|ToString(Integer) currentPitchId))
  (if (and (>= currentPitchId (Variables|Default|GetMinRangePitchId)) (<= currentPitchId (Variables|Default|GetMaxRangePitchId)))
    (Utilities|FlowControl|Sequence
      (:then_0
        (Rendering|Material|SetVectorParameterValue (Utilities|Array|Get(acopy) (Variables|Default|GetVisualCubes) (Variables|Default|GetLastNoteIndex)) "Color" (Math|Color|SelectColor :B "(R=0.000000,G=0.000000,B=0.000000,A=1.000000)" :bPickA true) :!class /Script/Engine.MaterialInstanceDynamic))
      (:then_1
        (Utilities|IsValid _currentnote
          (:Is%20Valid
            (bind _returnvalue (Class|SimplePitch|GetPitchId _currentnote))
            (if (>= _returnvalue 0)
              (Variables|Default|SetLastNoteIndex _returnvalue)
              (Rendering|Material|SetVectorParameterValue (Utilities|Array|Get(acopy) (Variables|Default|GetVisualCubes) _returnvalue) "Color" (Math|Color|SelectColor (Utilities|Array|Get(acopy) _visualcubescolors (Math|Random|RandomIntegerinRange 0 (- (Utilities|Array|Length _visualcubescolors) 1))) "(R=0.000000,G=0.000000,B=0.000000,A=1.000000)" true) :!class /Script/Engine.MaterialInstanceDynamic)
              (else
                (Development|PrintString "Incorrect pitch ID number" true true "(R=1.000000,G=0.000000,B=0.000000,A=1.000000)"))))
          (:Is%20Not%20Valid
            (Development|PrintString "Piano_Keyboard: Current note not valid" true true "(R=1.000000,G=0.000000,B=0.000000,A=1.000000)")))))))

(event EventBeginPlay
  (bind _outactors (Actor|GetAllActorsOfClass "/Game/Blueprints/BP_MicrophoneInput_Plus.BP_MicrophoneInput_Plus_C"))
  (Utilities|IsValid (Utilities|Array|Get(acopy) _outactors)
    (:Is%20Valid
      (bind _output_get (Variables|Default|SetMicrophoneInput (Utilities|Array|Get(acopy) _outactors)))
      (bind _output_get_2 (Variables|Default|SetPitchTracker (Variables|/Script/Midi_Project.MicrophoneInput|GetTracker _output_get)))
      (EventDispatchers|BindEventtoOnSoundRecordedDelegate _output_get_2 (delegate Custom|NewSoundInteraction))
      ;[1 1 1] Create Visual Cubes
      (for _index (range 0 115)
        (bind _returnvalue (AddComponent|AddStaticMeshComponent false (Math|Transform|MakeTransform (Math|Vector|MakeVector 0.0 (- (* _index 1e+01) 5.8e+02) 0.0) "0, 0, 0" "0.050000,0.050000,1.500000")))
        (bind _returnvalue_2 (Rendering|Material|CreateDynamicMaterialInstance _returnvalue 0 "/Game/Midi/Other/MatTest.MatTest" :!class /Script/Engine.PrimitiveComponent))
        (Utilities|Array|Add (Variables|Default|GetVisualCubes) _returnvalue_2))
      (for _index_2 (range 0 20)
        (Utilities|Array|Add (Variables|Default|GetVisualCubesColors) (Utilities|Struct|MakeLinearColor (Math|Random|RandomFloat) (Math|Random|RandomFloat) (Math|Random|RandomFloat) 1.0))))
    (:Is%20Not%20Valid
      (Development|PrintString "Piano_Keyboard: Microphone Input not valid" true true "(R=1.000000,G=0.000000,B=0.000000,A=1.000000)" 1e+01))))

(event Collision|EventActorBeginOverlap
  (params (OtherActor :type Actor%20Object%20Reference)))

(event EventTick
  (params (DeltaSeconds :type Float%20%28single-precision%29)))

(fn ConstructionScript)