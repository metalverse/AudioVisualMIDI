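; Musical interactive levitating sphere that opens once enough input of its ID-derived note accumulates.
; Opening blends material color and cover morph while spinning up, as the sphere follows its escape spline.
; It then closes interactive floor tiles and lerps to its ID-spaced start on the shared Levitating_Spheres_Orbit spline.
; Tick handles spin and orbiting, but the orbit trigger and laser beam creation are disconnected here.
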(event Custom|Escape
  (bind _levitatingsphere (Variables|Default|GetLevitatingSphere))
  (bind _levitatingsphere_2 (Variables|Default|GetLevitatingSphere))
  (bind _levitatingsphere_3 (Variables|Default|GetLevitatingSphere))
  (bind _escapepath (Variables|Default|GetEscapePath))
  (bind _returnvalue (Transformation|GetWorldTransform _levitatingsphere_2))
  (bind _returnvalue_2 (Transformation|GetWorldTransform _levitatingsphere_3))
  ;[1 1 1] Escape
  (bind _alpha (Timeline|Timeline_1 PlayFromStart)
    (:Update
      (Transformation|SetWorldTransform _levitatingsphere (Math|Transform|MakeTransform (Spline|GetLocationatDistanceAlongSpline _escapepath (* (Spline|GetSplineLength _escapepath) _alpha) "World") (Transformation|GetWorldRotation _levitatingsphere) (Transformation|GetWorldScale _levitatingsphere)) false false))
    (:Finished
      (CallFunction|CloseTiles)
      (Variables|Default|SetToOrbitStartPoint (.location _returnvalue_2))
      (Variables|Default|SetToOrbitStartRotation (.rotation _returnvalue_2))
      (bind _alpha_2 (Timeline|Timeline_2 PlayFromStart)
        (:Update
          (Transformation|SetWorldTransform _levitatingsphere_2 (Math|Transform|MakeTransform (Math|Vector|Lerp(Vector) (Variables|Default|GetToOrbitStartPoint) (Variables|Default|GetOrbitStartLocation) _alpha_2) (Math|Rotator|MakeRotator (.roll (.rotation _returnvalue)) (.pitch (Math|Rotator|Lerp(Rotator) (Variables|Default|GetToOrbitStartRotation) (Variables|Default|GetOrbitStartRotation) _alpha_2)) (.yaw (Math|Rotator|Lerp(Rotator) (Variables|Default|GetToOrbitStartRotation) (Variables|Default|GetOrbitStartRotation) _alpha_2))) (.scale _returnvalue)) false false))))))

(event Custom|Open
  ;[1 1 1] Open
  (bind (_direction _alpha _time) (Timeline|Timeline_0 PlayFromStart)
    (:Update
      (Rendering|Material|SetVectorParameterValue (Variables|Default|GetInsideMaterial) "Color" (Math|Color|Lerp(LinearColor) (Variables|Default|GetInactiveColor) (Variables|Default|GetActiveColor) _alpha) :!class /Script/Engine.MaterialInstanceDynamic)
      (Components|SkeletalMesh|SetMorphTarget (Variables|Default|GetLevitatingSphere) "Covers_Opened" _alpha true)
      (Transformation|AddLocalRotation (Variables|Default|GetLevitatingSphere) (Math|Rotator|MakeRotator (* (* _alpha (- _time (Variables|Default|GetLastTime))) (Variables|Default|GetAnglePerSecond)) 0.0 0.0) false false)
      (Variables|Default|SetLastTime _time))
    (:Finished
      (Variables|Default|SetShouldRotate true))))

(event EventBeginPlay
  ;[1 1 1] BeginPlay
  (Variables|Default|SetCurrentRotateAngle (.roll (Transformation|GetWorldRotation (Variables|Default|GetDefaultSceneRoot))))
  (bind _returnvalue (Rendering|Material|CreateDynamicMaterialInstance (Variables|Default|GetLevitatingSphere) 2 "/Game/Materials/LevitatingSphere/LevitatingSphere_Inactive.LevitatingSphere_Inactive" :!class /Script/Engine.PrimitiveComponent))
  (Variables|Default|SetInsideMaterial _returnvalue)
  (CallFunction|SetOrbitSpline))

(event Collision|EventActorBeginOverlap
  (params (OtherActor :type Actor%20Object%20Reference)))

(event EventTick
  (params (DeltaSeconds :type Float%20%28single-precision%29))
  (bind _orbit (Variables|Default|GetOrbit))
  (bind _levitatingsphere (Variables|Default|GetLevitatingSphere))
  (bind _returnvalue (Spline|GetSplineLength _orbit))
  ;[1 1 1] X Roll
  (Utilities|FlowControl|Sequence
    (:then_0
      (if (Variables|Default|GetShouldRotate)
        (Transformation|AddLocalRotation (Variables|Default|GetLevitatingSphere) (Math|Rotator|MakeRotator (* DeltaSeconds (Variables|Default|GetAnglePerSecond)) 0.0 0.0) false false)
        (Transformation|DetachFromActor "KeepWorld" "KeepWorld" "KeepWorld")))
    (:then_1
      ;[1 1 1] Orbiting
      (if (Variables|Default|GetIsOrbiting)
        (Transformation|SetWorldTransform _levitatingsphere (Math|Transform|MakeTransform (Spline|GetLocationatDistanceAlongSpline _orbit (Math|Float|%(Float) (+ (* (Variables|Default|GetOrbitCircuitPerSecond) DeltaSeconds _returnvalue) (Variables|Default|GetLastOrbitDistance)) _returnvalue) "World") (Math|Rotator|MakeRotator (.roll (Transformation|GetWorldRotation _levitatingsphere)) (.pitch (Spline|GetRotationatDistanceAlongSpline _orbit (Math|Float|%(Float) (+ (* (Variables|Default|GetOrbitCircuitPerSecond) DeltaSeconds _returnvalue) (Variables|Default|GetLastOrbitDistance)) _returnvalue) "World")) (.yaw (Spline|GetRotationatDistanceAlongSpline _orbit (Math|Float|%(Float) (+ (* (Variables|Default|GetOrbitCircuitPerSecond) DeltaSeconds _returnvalue) (Variables|Default|GetLastOrbitDistance)) _returnvalue) "World"))) (Transformation|GetWorldScale _levitatingsphere)) false false)
        (Variables|Default|SetLastOrbitDistance (Math|Float|%(Float) (+ (* (Variables|Default|GetOrbitCircuitPerSecond) DeltaSeconds _returnvalue) (Variables|Default|GetLastOrbitDistance)) _returnvalue))))))

(event EventHandleInputNoteId
  (params (NoteId :type Integer) (Value :type Integer))
  ;[1 1 1] Interaction
  (|CallParentFunction NoteId Value)
  (if (not (Variables|Default|GetAlreadyOpened))
    (if (== (Math|Integer|%(Integer) NoteId 12) (Variables|Default|GetInteractionTone))
      (bind _output_get (Variables|Default|SetReceivedValue (+ Value (Variables|Default|GetReceivedValue))))
      (Development|PrintString (Utilities|String|Append (Utilities|String|ToString(Float) (/ (* _output_get 1e+02) (Math|Conversions|ToFloat(Integer) (Variables|Default|GetValueNeededForInteraction)))) "%"))
      (if (> (Variables|Default|GetReceivedValue) (Variables|Default|GetValueNeededForInteraction))
        (Variables|Default|SetAlreadyOpened true)
        (Transformation|DetachFromActor "KeepWorld" "KeepWorld" "KeepWorld")
        (CallFunction|Open)
        (CallFunction|Escape))
      (else
        (bind _alpha (Timeline|Timeline_3 PlayFromStart)
          (:Update
            (Rendering|Material|SetVectorParameterValue (Variables|Default|GetInsideMaterial) "Color" (Math|Color|Lerp(LinearColor) (Variables|Default|GetActiveColor) (Variables|Default|GetInactiveColor) _alpha) :!class /Script/Engine.MaterialInstanceDynamic)))))))

(fn ConstructionScript
  (bind _output_get (Variables|Default|SetInteractionTone (* (Variables|Default|GetID) 4)))
  (bind _notecolor (CallFunction|GetColorbyNoteId _output_get))
  (Variables|Default|SetActiveColor _notecolor))

(fn SetOrbitSpline
  (bind _outactors (Actor|GetAllActorsOfClass "/Game/Blueprints/Levitating_Spheres_Orbit.Levitating_Spheres_Orbit_C"))
  (Utilities|IsValid (Utilities|Array|Get(acopy) _outactors)
    (:Is%20Valid
      (bind _output_get (Variables|Default|SetOrbit (Variables|/Game/Blueprints/Levitating_Spheres_Orbit.Levitating_Spheres_Orbit_C|GetOrbit (Utilities|Array|Get(acopy) _outactors))))
      (bind _output_get_2 (Variables|Default|SetOrbitOffset (* (Variables|Default|GetID) (/ (Spline|GetSplineLength _output_get) 3.0))))
      (bind _output_get_3 (Variables|Default|SetLastOrbitDistance _output_get_2))
      (Variables|Default|SetOrbitStartLocation (Spline|GetLocationatDistanceAlongSpline (Variables|Default|GetOrbit) (Math|Float|%(Float) _output_get_3 (Spline|GetSplineLength (Variables|Default|GetOrbit))) "World"))
      (Variables|Default|SetOrbitStartRotation (Spline|GetRotationatDistanceAlongSpline (Variables|Default|GetOrbit) (Math|Float|%(Float) _output_get_3 (Spline|GetSplineLength (Variables|Default|GetOrbit))) "World")))
    (:Is%20Not%20Valid
      (Development|PrintString "Orbit not valid!" true true "(R=1.000000,G=0.000000,B=0.000000,A=1.000000)" 1e+01))))

(fn CreateBeam
  (bind _returnvalue (Game|SpawnActorfromClass "/Game/Blueprints/Laser_Beam.Laser_Beam_C" (Transformation|GetSocketTransform (Variables|Default|GetLevitatingSphere) "Emitter1" "RTS_Component") "Undefined" 0 0))
  (bind _output_get (Variables|Default|SetLaserBeam _returnvalue))
  (Transformation|AttachComponentToComponent _output_get (Variables|Default|GetLevitatingSphere) "Emitter1" "KeepRelative" "KeepRelative" "KeepRelative" true)
  (Class|ParticleSystemComponent|SetBeamTargetPoint (Variables|/Game/Blueprints/Laser_Beam.Laser_Beam_C|GetLaserParticleSystem (Variables|Default|GetLaserBeam)) 0 "0, 0,540.000000")
  (Default|SetBeamColor (Variables|Default|GetLaserBeam) (Variables|Default|GetActiveColor)))

(fn CloseTiles
  (bind _asfirst_person_character (Utilities|Casting|CastToFirstPersonCharacter (Game|GetPlayerCharacter 0)))
  (for _array_element (Variables|/Game/FirstPersonBP/Blueprints/FirstPersonCharacter.FirstPersonCharacter_C|GetActorsIgnoredForTracing _asfirst_person_character)
    (bind _assio_hex_floor_tile_interactive (Utilities|Casting|CastToSIO_Hex_Floor_Tile_Interactive _array_element))
    (Default|Close _assio_hex_floor_tile_interactive)))