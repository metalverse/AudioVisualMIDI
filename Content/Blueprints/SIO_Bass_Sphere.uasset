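; Interactive bass sound object with a sphere and morphing pyramid that visualizes MIDI notes and can be played by player input, apparently voice.
; Open animates the pyramid and starts the MIDI manager's track.
; Note events drive sphere color, scale and morph through timelines.
; Onset counts switch interaction modes, toggling the file's channel; input notes play an octave lower and are mirrored to all levitating spheres.
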(event Custom|Open
  (bind _pyramidmesh (Variables|Default|GetPyramidMesh))
  ;[1 1 1] Open
  (Variables|Default|SetPlayerInteractive true)
  (Utilities|FlowControl|Sequence
    (:then_0
      (bind _alpha (Timeline|Timeline_0 PlayFromStart)
        (:Update
          (Components|SkeletalMesh|SetMorphTarget (Variables|Default|GetPyramidMesh) "Activating" _alpha true))
        (:Finished
          (bind _alpha_2 (Timeline|Timeline_1 PlayFromStart)
            (:Update
              (Components|SkeletalMesh|SetMorphTarget _pyramidmesh "Open" (* _alpha_2 1.2) true)
              (Components|SkeletalMesh|SetMorphTarget _pyramidmesh "Activating" (- 1.0 _alpha_2) true)
              (Rendering|Material|SetVectorParameterValue (Variables|Default|GetPyramidMaterial) "Color" (Math|Color|Lerp(LinearColor) (Variables|Default|GetActionColor) (Variables|Default|GetIdleColor) _alpha_2) :!class /Script/Engine.MaterialInstanceDynamic))
            (:Finished
              (Variables|Default|SetActorLocation (Transformation|GetWorldLocation (Variables|Default|GetBassSphereMesh))))))))
    (:then_1
      (Utilities|FlowControl|Delay 3.3)
      (bind _outactors (Actor|GetAllActorsOfClass "/Game/Blueprints/BP_MidiManager.BP_MidiManager_C"))
      (Default|PlayTrack (Utilities|Array|Get(acopy) _outactors)))))

(event EventBeginPlay
  ;[1 1 1] Begin Play
  (bind _returnvalue (Rendering|Material|CreateDynamicMaterialInstance (Variables|Default|GetBassSphereMesh) 0 "/Game/Materials/MatTest.MatTest" :!class /Script/Engine.PrimitiveComponent))
  (Variables|Default|SetSphereMaterial _returnvalue)
  (Utilities|FlowControl|Delay 6.0)
  (bind _returnvalue_2 (Rendering|Material|CreateDynamicMaterialInstance (Variables|Default|GetPyramidMesh) 1 "/Game/Materials/MatTest.MatTest" :!class /Script/Engine.PrimitiveComponent))
  (Variables|Default|SetPyramidMaterial _returnvalue_2)
  (bind _outactors (Actor|GetAllActorsOfClass "/Game/Blueprints/SIO_Levitating_Sphere.SIO_Levitating_Sphere_C"))
  (Variables|Default|SetLevitatingSpheres _outactors)
  (Variables|Default|SetActorLocation (Transformation|GetWorldLocation (Variables|Default|GetBassSphereMesh)))
  (bind _outactors_2 (Actor|GetAllActorsOfClass "/Game/Blueprints/BP_MidiManager.BP_MidiManager_C"))
  (Utilities|IsValid (Utilities|Array|Get(acopy) _outactors_2)
    (:Is%20Valid
      (Variables|Default|SetVisual_Midi (Utilities|Array|Get(acopy) _outactors_2)))))

(event Collision|EventActorBeginOverlap
  (params (OtherActor :type Actor%20Object%20Reference)))

(event EventHandleInputNoteId
  (params (NoteId :type Integer) (Value :type Integer))
  (bind _visual_midi (Variables|Default|GetVisual_Midi))
  ;[1 1 1] Handle Input Note Id
  (if (or (Utilities|Enum|Equal(Enum) (Variables|Default|GetInteractionMode) "NewEnumerator1") (Utilities|Enum|Equal(Enum) (Variables|Default|GetInteractionMode) "NewEnumerator0"))
    (if (!= (- NoteId 12) (Variables|Default|GetCurrentNotePlaying))
      (Default|StopMidiNoteonChannel _visual_midi (Variables|Default|GetInstrumentChannel) (Variables|Default|GetCurrentNotePlaying))
      (bind _output_get (Variables|Default|SetCurrentNotePlaying (- NoteId 12)))
      (Default|PlayMidiNoteonChannel _visual_midi (Variables|Default|GetInstrumentChannel) _output_get)
      (CallFunction|VoiceInteraction _output_get 3500 (Variables|Default|GetMidiNoteOn))
      (for _array_element (Variables|Default|GetLevitatingSpheres)
        (Default|VoiceInteraction _array_element _output_get 3500 (Variables|Default|GetMidiNoteOn))))))

(event EventHandleInputOnset
  ;[1 1 1] Handle Input Onset
  (|CallParentFunction)
  (Development|PrintString (Utilities|String|ToString(Integer) (Variables|Default|GetDetectedInteractionOnsets)) true true "(R=1.000000,G=0.879220,B=0.000000,A=1.000000)" 4.0))

(event EventMidiInteraction
  (params (CurrentNote :type Integer) (NextNote :type Integer) (TimeDifference :type Integer) (EventType :type Integer))
  (bind _basescale (Variables|Default|GetBaseScale))
  ;[1 1 1] Midi Interaction
  (if (not (Math|Boolean|ORBoolean (Variables|Default|GetIsInInteractiveMode) (not (Utilities|Enum|Equal(Enum) (Variables|Default|GetInteractionMode) "NewEnumerator2")) (Utilities|Enum|Equal(Enum) (Variables|Default|GetInteractionMode) "NewEnumerator3")))
    (Variables|Default|SetCurrentNoteID CurrentNote)
    (Variables|Default|SetCurrentTimeDifference TimeDifference)
    (Variables|Default|SetCurrentEventType EventType)
    (bind _notecolor (CallFunction|GetColorbyNoteId (Variables|Default|GetCurrentNoteID)))
    (Variables|Default|SetActionColor _notecolor)
    (if (== (Variables|Default|GetCurrentEventType) (Variables|Default|GetMidiNoteOn))
      (Components|Timeline|SetPlayRate (Variables|Default|GetSmoothColorLerp) (/ 1.0 (/ (Math|Conversions|ToFloat(Integer) (Variables|Default|GetCurrentTimeDifference)) 1e+03)))
      (bind _alpha (Timeline|SmoothColorLerp PlayFromStart)
        (:Update
          (Variables|Default|SetCurrentAlpha _alpha)
          (Rendering|Material|SetVectorParameterValue (Variables|Default|GetSphereMaterial) "Color" (Math|Color|Lerp(LinearColor) (Variables|Default|GetActionColor) (Variables|Default|GetIdleColor) _alpha) :!class /Script/Engine.MaterialInstanceDynamic)
          (Transformation|SetWorldScale3D (Variables|Default|GetBassSphereMesh) (+ (* _basescale (* (- 1.0 _alpha) 0.6)) _basescale))
          (Components|SkeletalMesh|SetMorphTarget (Variables|Default|GetBassSphereMesh) "Closed" (* _alpha 0.5) true))))))

(event EventTick
  (params (DeltaSeconds :type Float%20%28single-precision%29)))

(event EventHandleInputSilence
  (bind _basescale (Variables|Default|GetBaseScale))
  (bind _basescale_2 (Variables|Default|GetBaseScale))
  ;[1 1 1] Handle Input Silence
  (if (or (Utilities|Enum|Equal(Enum) (Variables|Default|GetInteractionMode) "NewEnumerator1") (Utilities|Enum|Equal(Enum) (Variables|Default|GetInteractionMode) "NewEnumerator0"))
    (Utilities|FlowControl|Sequence
      (:then_0
        ;[1 1 1] Midi Interaction
        (bind _alpha (Timeline|SmoothColorLerp Stop)
          (:Update
            (Variables|Default|SetCurrentAlpha _alpha)
            (Rendering|Material|SetVectorParameterValue (Variables|Default|GetSphereMaterial) "Color" (Math|Color|Lerp(LinearColor) (Variables|Default|GetActionColor) (Variables|Default|GetIdleColor) _alpha) :!class /Script/Engine.MaterialInstanceDynamic)
            (Transformation|SetWorldScale3D (Variables|Default|GetBassSphereMesh) (+ (* _basescale_2 (* (- 1.0 _alpha) 0.6)) _basescale_2))
            (Components|SkeletalMesh|SetMorphTarget (Variables|Default|GetBassSphereMesh) "Closed" (* _alpha 0.5) true))))
      (:then_1
        (Components|Timeline|SetPlayRate (Variables|Default|GetSmoothLerpSilence) 2.0)
        (bind _alpha_2 (Timeline|SmoothLerpSilence PlayFromStart)
          (:Update
            (Rendering|Material|SetVectorParameterValue (Variables|Default|GetSphereMaterial) "Color" (Math|Color|Lerp(LinearColor) (Variables|Default|GetActionColor) (Variables|Default|GetIdleColor) (Math|Float|Lerp (Variables|Default|GetCurrentAlpha) 1.0 _alpha_2)) :!class /Script/Engine.MaterialInstanceDynamic)
            (Transformation|SetWorldScale3D (Variables|Default|GetBassSphereMesh) (+ (* _basescale (* (- 1.0 (Math|Float|Lerp (Variables|Default|GetCurrentAlpha) 1.0 _alpha_2)) 0.6)) _basescale))
            (Components|SkeletalMesh|SetMorphTarget (Variables|Default|GetBassSphereMesh) "Closed" (* (Math|Float|Lerp (Variables|Default|GetCurrentAlpha) 1.0 _alpha_2) 0.5) true))
          (:Finished
            (Default|StopMidiNoteonChannel (Variables|Default|GetVisual_Midi) (Variables|Default|GetInstrumentChannel) (Variables|Default|GetCurrentNotePlaying))
            (Variables|Default|SetCurrentNotePlaying 0))))
      (:then_2
        (for _array_element (Variables|Default|GetLevitatingSpheres)
          (Default|StopVoiceInteraction _array_element))))))

(event EventVoiceInteraction
  (params (MidiNote :type Integer) (TimeDifference :type Integer) (EventType :type Integer))
  (bind _basescale (Variables|Default|GetBaseScale))
  ;[1 1 1] Midi Interaction
  ;;[1 1 1] Voice Interaction
  (Variables|Default|SetCurrentNoteID MidiNote)
  (Variables|Default|SetCurrentTimeDifference TimeDifference)
  (Variables|Default|SetCurrentEventType EventType)
  (bind _notecolor (CallFunction|GetColorbyNoteId (Variables|Default|GetCurrentNoteID)))
  (Variables|Default|SetActionColor _notecolor)
  (if (== (Variables|Default|GetCurrentEventType) (Variables|Default|GetMidiNoteOn))
    (Components|Timeline|SetPlayRate (Variables|Default|GetSmoothColorLerp) (/ 1.0 (/ (Math|Conversions|ToFloat(Integer) (Variables|Default|GetCurrentTimeDifference)) 1e+03)))
    (bind _alpha (Timeline|SmoothColorLerp PlayFromStart)
      (:Update
        (Variables|Default|SetCurrentAlpha _alpha)
        (Rendering|Material|SetVectorParameterValue (Variables|Default|GetSphereMaterial) "Color" (Math|Color|Lerp(LinearColor) (Variables|Default|GetActionColor) (Variables|Default|GetIdleColor) _alpha) :!class /Script/Engine.MaterialInstanceDynamic)
        (Transformation|SetWorldScale3D (Variables|Default|GetBassSphereMesh) (+ (* _basescale (* (- 1.0 _alpha) 0.6)) _basescale))
        (Components|SkeletalMesh|SetMorphTarget (Variables|Default|GetBassSphereMesh) "Closed" (* _alpha 0.5) true)))))

(event EventChooseInteractionMode
  (bind _visual_midi (Variables|Default|GetVisual_Midi))
  (bind _basescale (Variables|Default|GetBaseScale))
  ;[1 1 1] Choose Interaction Mode
  (|CallParentFunction)
  (switch int (Variables|Default|GetDetectedInteractionOnsets)
    (:1
      (CallFunction|HandleInteractiveModeon))
    (:2
      (CallFunction|HandleInteractiveModeon))
    (:3
      (Variables|Default|SetCanInteract false)
      (Utilities|Time|SetTimerbyFunctionName 0 "ReleaseInteraction" 1.0)
      (if (Utilities|Enum|Equal(Enum) (Variables|Default|GetInteractionMode) "NewEnumerator2")
        (Default|IncludeChanneltoFileData _visual_midi (Utilities|Array|MakeArray (Variables|Default|GetInstrumentChannel)))
        (for _array_element (Variables|Default|GetLevitatingSpheres)
          (Variables|/Game/Blueprints/BP_Sound_Interactive_Object.BP_Sound_Interactive_Object_C|SetIsInInteractiveMode _array_element false)
          (Default|AllChannelsonSameLevel _visual_midi)
          (for _array_element_2 (Variables|Default|GetLevitatingSpheres)
            (Variables|/Game/Blueprints/BP_Sound_Interactive_Object.BP_Sound_Interactive_Object_C|SetInteractionMode _array_element_2 (Variables|Default|GetInteractionMode)))
          (Variables|Default|SetIsInInteractiveMode false))
        (else
          (Utilities|FlowControl|Sequence
            (:then_0
              (for _array_element_3 (Variables|Default|GetLevitatingSpheres)
                (Variables|/Game/Blueprints/BP_Sound_Interactive_Object.BP_Sound_Interactive_Object_C|SetIsInInteractiveMode _array_element_3 true)
                (Default|StopVoiceInteraction _array_element_3)
                (for _array_element_4 (Variables|Default|GetLevitatingSpheres)
                  (Variables|/Game/Blueprints/BP_Sound_Interactive_Object.BP_Sound_Interactive_Object_C|SetInteractionMode _array_element_4 (Variables|Default|GetInteractionMode)))
                (Variables|Default|SetIsInInteractiveMode false)))
            (:then_1
              (Default|ExcludeChannelfromFileData (Variables|Default|GetVisual_Midi) (Utilities|Array|MakeArray (Variables|Default|GetInstrumentChannel)))
              ;[1 1 1] Handle Input Silence
              (bind _alpha (Timeline|SmoothLerpSilence PlayFromStart)
                (:Update
                  (Rendering|Material|SetVectorParameterValue (Variables|Default|GetSphereMaterial) "Color" (Math|Color|Lerp(LinearColor) (Variables|Default|GetActionColor) (Variables|Default|GetIdleColor) (Math|Float|Lerp (Variables|Default|GetCurrentAlpha) 1.0 _alpha)) :!class /Script/Engine.MaterialInstanceDynamic)
                  (Transformation|SetWorldScale3D (Variables|Default|GetBassSphereMesh) (+ (* _basescale (* (- 1.0 (Math|Float|Lerp (Variables|Default|GetCurrentAlpha) 1.0 _alpha)) 0.6)) _basescale))
                  (Components|SkeletalMesh|SetMorphTarget (Variables|Default|GetBassSphereMesh) "Closed" (* (Math|Float|Lerp (Variables|Default|GetCurrentAlpha) 1.0 _alpha) 0.5) true))
                (:Finished
                  (Default|StopMidiNoteonChannel (Variables|Default|GetVisual_Midi) (Variables|Default|GetInstrumentChannel) (Variables|Default|GetCurrentNotePlaying))
                  (Variables|Default|SetCurrentNotePlaying 0))))))))))

(event EventHandleOnsetChangeInteraction
  (bind _visual_midi (Variables|Default|GetVisual_Midi))
  ;[1 1 1] Handle Onset Change Interaction
  (|CallParentFunction)
  (switch int (Variables|Default|GetDetectedInteractionOnsets)
    (:1
      (if (Utilities|Enum|Equal(Enum) (Variables|Default|GetInteractionMode) "NewEnumerator1")
        (CallFunction|SetInstrumentbyLastNote)))
    (:2
      (Variables|Default|SetCanInteract false)
      (Utilities|Time|SetTimerbyFunctionName 0 "ReleaseInteraction" 1.0)
      (for _array_element (Variables|Default|GetLevitatingSpheres)
        (Variables|/Game/Blueprints/BP_Sound_Interactive_Object.BP_Sound_Interactive_Object_C|SetIsInInteractiveMode _array_element false))
      (Default|IncludeChanneltoFileData _visual_midi (Utilities|Array|MakeArray (Variables|Default|GetInstrumentChannel)))
      (Default|AllChannelsonSameLevel _visual_midi))))

(fn ConstructionScript)

(fn HandleInteractiveModeon
  (Utilities|FlowControl|Sequence
    (:then_0
      (Default|ExcludeChannelfromFileData (Variables|Default|GetVisual_Midi) (Utilities|Array|MakeArray (Variables|Default|GetInstrumentChannel)))
      (Default|HandleChannelonFirstPlace (Variables|Default|GetVisual_Midi) (Variables|Default|GetInstrumentChannel))
      (Rendering|Material|SetVectorParameterValue (Variables|Default|GetSphereMaterial) "Color" (Variables|Default|GetIdleColor) :!class /Script/Engine.MaterialInstanceDynamic)
      (Transformation|SetWorldScale3D (Variables|Default|GetBassSphereMesh) (Variables|Default|GetBaseScale))
      (Components|SkeletalMesh|SetMorphTarget (Variables|Default|GetBassSphereMesh) "Closed" 0.5 true))
    (:then_1
      (for _array_element (Variables|Default|GetLevitatingSpheres)
        (Variables|/Game/Blueprints/BP_Sound_Interactive_Object.BP_Sound_Interactive_Object_C|SetIsInInteractiveMode _array_element true)
        ;[1 1 1] For clearing previous animation
        (Default|StopVoiceInteraction _array_element)))))