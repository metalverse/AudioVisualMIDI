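; Base sound-interactive hex floor tile that changes its material color in response to microphone input.
; Binds to the Sound component of BP_MicrophoneInput_Plus, coloring by pitch for notes and using a separate flash color for volume onsets.
; Reacts only when volume outweighs player distance, with timers delayed by distance so sound ripples outward from the player.
; Timelines blend between pitches and fade to idle; waiting flags handle notes ending before the delayed reaction.
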(event Custom|ReactOnSoundModify
  ;[1 1 1] React On Sound Modify
  (Variables|Default|SetIsInSoundMode true)
  (bind _notecolor (CallFunction|GetColorbyNoteId (Variables|Default|GetCurrentPitchId)))
  (bind _output_get (Variables|Default|SetTemporaryColor (Variables|Default|GetGlobalInteractionColor)))
  (bind _alpha (Timeline|Timeline_2 PlayFromStart)
    (:Update
      (bind _output_get_2 (Variables|Default|SetGlobalInteractionColor (Math|Color|Lerp(LinearColor) _output_get _notecolor _alpha)))
      (Rendering|Material|SetVectorParameterValue (Variables|Default|GetMaterial) "Color" _output_get_2 :!class /Script/Engine.MaterialInstanceDynamic))))

(event Custom|ReactOnSoundOn
  ;[1 1 1] React On Sound
  (Variables|Default|SetWaitingForNoteOn false)
  (Utilities|FlowControl|Sequence
    (:then_0
      ;[1 1 1] React On Sound Off
      (bind _alpha (Timeline|Timeline_0 Stop)
        (:Update
          (Rendering|Material|SetVectorParameterValue (Variables|Default|GetMaterial) "Color" (Math|Color|Lerp(LinearColor) (Variables|Default|GetGlobalInteractionColor) (Variables|Default|GetIdleColor) _alpha) :!class /Script/Engine.MaterialInstanceDynamic))))
    (:then_1
      (Variables|Default|SetIsInSoundMode true)
      (Rendering|Material|SetVectorParameterValue (Variables|Default|GetMaterial) "Color" (Variables|Default|GetGlobalInteractionColor) :!class /Script/Engine.MaterialInstanceDynamic)
      (if (Variables|Default|GetWaitingForNoteOff)
        (CallFunction|ReactonSoundOff)))))

(event Custom|SoundDetectedEvent
  (params (mode :type Integer) (value :type Integer) (pitchId :type Integer) (volume :type Float%20%28single-precision%29))
  (bind _soundeventmodes (Variables|Default|GetSoundEventModes))
  ;[1 1 1] Sound Detected Event
  (if (== mode (.soundon _soundeventmodes))
    (bind (_shouldreact _timeforreaction) (CallFunction|ShouldReactonSound volume :!label _label))
    (if _shouldreact
      (Variables|Default|SetCurrentPitchId pitchId)
      (bind _notecolor (CallFunction|GetColorbyNoteId pitchId))
      (Variables|Default|SetGlobalInteractionColor _notecolor)
      (Variables|Default|SetWaitingForNoteOn true)
      (Utilities|Time|SetTimerbyEvent (delegate Custom|ReactOnSoundOn) _timeforreaction))
    (elif (== mode (.soundoff _soundeventmodes))
      (if (Variables|Default|GetIsInSoundMode)
        (Variables|Default|SetIsInSoundMode false)
        (CallFunction|ReactonSoundOff)
        (elif (Variables|Default|GetWaitingForNoteOn)
          (Variables|Default|SetWaitingForNoteOff true)))
      (elif (== mode (.soundmodify _soundeventmodes))
        (Variables|Default|SetCurrentPitchId pitchId)
        (if (Variables|Default|GetIsInSoundMode)
          (bind _shouldreact_2 (CallFunction|ShouldReactonSound volume))
          (if _shouldreact_2
            (CallFunction|ReactonSoundModify)
            (else
              (CallFunction|ReactonSoundOff)))
          (elif (not (Variables|Default|GetWaitingForNoteOn))
            (goto _label)))
        (elif (== mode (.volumeevent _soundeventmodes))
          (if (not (Variables|Default|GetIsInSoundMode))
            (bind (_shouldreact_3 _timeforreaction_2) (CallFunction|ShouldReactonSound volume))
            (if _shouldreact_3
              (Variables|Default|SetIsInSoundMode true)
              (Utilities|Time|SetTimerbyEvent (delegate Custom|ReactOnOnsetOn) _timeforreaction_2)
              (Utilities|Time|SetTimerbyEvent (delegate Custom|ReactOnOnsetOff) (+ _timeforreaction_2 0.3)))))))))

(event Custom|ReactOnOnsetOn
  ;[1 1 1] React On Onset On
  (Variables|Default|SetIsInSoundMode true)
  (Rendering|Material|SetVectorParameterValue (Variables|Default|GetMaterial) "Color" (Variables|Default|GetOnsetInteractionColor) :!class /Script/Engine.MaterialInstanceDynamic))

(event Custom|ReactOnOnsetOff
  ;[1 1 1] React On Onset Off
  (bind _alpha (Timeline|Timeline_1 PlayFromStart)
    (:Update
      (Rendering|Material|SetVectorParameterValue (Variables|Default|GetMaterial) "Color" (Math|Color|Lerp(LinearColor) (Variables|Default|GetOnsetInteractionColor) (Variables|Default|GetIdleColor) _alpha) :!class /Script/Engine.MaterialInstanceDynamic)
      (Variables|Default|SetIsInSoundMode false))))

(event Custom|ReactOnSoundOff
  ;[1 1 1] React On Sound Off
  (Variables|Default|SetWaitingForNoteOff false)
  (Variables|Default|SetIsInSoundMode false)
  (bind _alpha (Timeline|Timeline_0 PlayFromStart)
    (:Update
      (Rendering|Material|SetVectorParameterValue (Variables|Default|GetMaterial) "Color" (Math|Color|Lerp(LinearColor) (Variables|Default|GetGlobalInteractionColor) (Variables|Default|GetIdleColor) _alpha) :!class /Script/Engine.MaterialInstanceDynamic))))

(event EventBeginPlay
  ;[1 1 1] Begin Play
  (bind _outactors (Actor|GetAllActorsOfClass "/Game/Blueprints/BP_MicrophoneInput_Plus.BP_MicrophoneInput_Plus_C"))
  (Utilities|IsValid (Utilities|Array|Get(acopy) _outactors)
    (:Is%20Valid
      (bind _output_get (Variables|Components|SetSoundComponent (Variables|/Game/Blueprints/BP_MicrophoneInput_Plus.BP_MicrophoneInput_Plus_C|GetSound (Utilities|Array|Get(acopy) _outactors))))
      (EventDispatchers|BindEventtoOnEventSoundDetected _output_get (delegate Custom|SoundDetectedEvent)))
    (:Is%20Not%20Valid
      (Development|PrintString "SIO_Floating: MicrophoneInput not valid" true true "(R=1.000000,G=0.000000,B=0.000000,A=1.000000)" 1e+01))))

(event Collision|EventActorBeginOverlap
  (params (OtherActor :type Actor%20Object%20Reference)))

(event EventHandleInputNoteId
  (params (NoteId :type Integer) (Value :type Integer)))

(event EventTick
  (params (DeltaSeconds :type Float%20%28single-precision%29)))

(fn ConstructionScript)

(fn ShouldReactonSound
  (params (Volume :type Float%20%28single-precision%29))
  (bind _returnvalue (Game|Player|GetPlayerPawn 0))
  (bind _maxinteractiondistance (Variables|Default|GetMaxInteractionDistance))
  (bind _actorlocation (Variables|Default|GetActorLocation))
  (bind _returnvalue_2 (Transformation|GetActorLocation _returnvalue))
  (bind _returnvalue_3 (- _returnvalue_2 _actorlocation))
  (bind _returnvalue_4 (Math|Vector|VectorLength _returnvalue_3))
  (if (< _returnvalue_4 _maxinteractiondistance)
    (if (> (Math|Float|Clamp(Float) (Math|Float|NormalizetoRange Volume 4.0 (Variables|Default|GetMaxDistanceVolume))) (Math|Float|Clamp(Float) (Math|Float|NormalizetoRange _returnvalue_4 0.0 _maxinteractiondistance)))
      (return true (/ _returnvalue_4 (Variables|Default|GetDelayDistanceDevider)))
      (else
        _)))
  (return false 0.0))

(fn GetReactDelay
  (return (/ (Math|Vector|VectorLength (- (Transformation|GetActorLocation (Game|Player|GetPlayerPawn 0)) (Variables|Default|GetActorLocation))) (Variables|Default|GetDelayDistanceDevider))))