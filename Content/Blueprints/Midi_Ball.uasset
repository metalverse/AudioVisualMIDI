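; Midi Ball actor that slides its Sphere along the local Y axis to follow incoming MIDI values.
; UpdatePosition takes a value and a time in milliseconds, then shifts the target by ten units per MIDI step of change.
; The SmoothMooving timeline has its play rate scaled by that time and interpolates the sphere from the previous target to the new one.
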(event Custom|UpdatePosition
  (params (MidiValue :type Integer) (Time :type Integer))
  (CallFunction|UpdateStartLocations MidiValue)
  (Components|Timeline|SetPlayRate (Variables|Default|GetSmoothMooving) (/ 1.0 (/ (Math|Conversions|ToFloat(Integer) Time) 1e+03)))
  (bind _position (Timeline|SmoothMooving PlayFromStart)
    (:Update
      (CallFunction|UpdateCurrentPosition _position))))

(event EventBeginPlay
  (bind _output_get (Variables|Default|SetStartLocation (Variables|/Script/Engine.SceneComponent|GetRelativeLocation (Variables|Default|GetSphere))))
  (Variables|Default|SetTargetLocation _output_get))

(event Collision|EventActorBeginOverlap
  (params (OtherActor :type Actor%20Object%20Reference)))

(event EventTick
  (params (DeltaSeconds :type Float%20%28single-precision%29)))

(fn ConstructionScript)

(fn ChangeTarget)

(fn UpdateStartLocations
  (params (NewMidiValue :type Integer))
  (Variables|Default|SetstartMidiValue (Variables|Default|GettargetMidiValue))
  (Variables|Default|SettargetMidiValue NewMidiValue)
  (Variables|Default|SetStartLocation (Variables|Default|GetTargetLocation))
  (Variables|Default|SetTargetLocation (+ (Variables|Default|GetStartLocation) (Math|Vector|MakeVector 0.0 (* (- (Variables|Default|GettargetMidiValue) (Variables|Default|GetstartMidiValue)) 1e+01) 0.0))))

(fn UpdateCurrentPosition
  (params (Alpha :type Float%20%28single-precision%29))
  (Transformation|SetRelativeLocation (Variables|Default|GetSphere) (+ (Variables|Default|GetStartLocation) (Math|Vector|MakeVector 0.0 (* Alpha (* (- (Variables|Default|GettargetMidiValue) (Variables|Default|GetstartMidiValue)) 1e+01)) 0.0)) false false))