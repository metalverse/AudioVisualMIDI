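; Sound-interactive hex floor edge tile bound to one pitch class, which flashes that note's color and pulses in height when a matching note plays.
; It listens to MIDI and wall-interaction events from BP_Microphone_Input's sound component, sharing mode changes through that component.
; Detected onset counts switch between control, edit, normal and disabled modes.
; In control or edit mode, input notes play through BP_MidiManager, which also includes or excludes the channel from file playback.
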(event Custom|HandleWallInteraction
  (params (isActive :type Boolean) (mode :type Integer) (noteId :type Integer))
  (bind _returnvalue (Math|Integer|%(Integer) noteId 12))
  (Variables|Default|SetIsInInteractiveMode isActive)
  (switch int mode
    (:0
      (Variables|Default|SetInteractionMode "NewEnumerator0"))
    (:1
      (Variables|Default|SetInteractionMode "NewEnumerator1"))
    (:2
      (Variables|Default|SetInteractionMode "NewEnumerator2"))
    (:3
      (Variables|Default|SetInteractionMode "NewEnumerator3")))
  (if (>= noteId 0)
    (bind _output_get (Variables|Default|SetCurrentNotePlaying noteId))
    (Variables|Default|SetNoteToStop _output_get)
    (if (and (== _returnvalue (Variables|Default|GetInteractionPitchId)) (!= _returnvalue (Variables|Default|GetCurrentNotePlaying)))
      (CallFunction|VoiceInteraction noteId 1750 (Variables|Default|GetMidiNoteOn)))
    (elif (== noteId -2)
      (Variables|Default|SetCurrentNotePlaying 0))))

(event Custom|MidiInteractionEvent
  (params (channel :type Integer) (noteId :type Integer) (timeDifference :type Integer) (type :type Integer))
  ;[1 1 1] Midi Interaction
  (if (not (Variables|Default|GetIsInInteractiveMode))
    (if (== channel (Variables|Default|GetInstrumentChannel))
      (if (== (Math|Integer|%(Integer) noteId 12) (Variables|Default|GetInteractionPitchId))
        (Variables|Default|SetCurrentNoteID noteId)
        (Variables|Default|SetCurrentTimeDifference timeDifference)
        (Variables|Default|SetCurrentEventType type)
        (if (== (Variables|Default|GetCurrentEventType) (Variables|Default|GetMidiNoteOn))
          (Components|Timeline|SetPlayRate (Variables|Default|GetSmoothColorLerp) (/ 1.0 (/ (Math|Conversions|ToFloat(Integer) (Variables|Default|GetCurrentTimeDifference)) 1e+03)))
          (bind _alpha (Timeline|SmoothColorLerp PlayFromStart)
            (:Update
              (Rendering|Material|SetVectorParameterValue (Variables|Default|GetMaterial) "Color" (Math|Color|Lerp(LinearColor) (Variables|Default|GetGlobalInteractionColor) (Variables|Default|GetIdleColor) _alpha) :!class /Script/Engine.MaterialInstanceDynamic)
              (Transformation|SetWorldScale3D (Variables|Default|GetFrequency) (Math|Vector|Lerp(Vector) (- (Variables|Default|GetBaseScale) (* (Math|Vector|MakeVector 0.0 0.0 (.z (Variables|Default|GetBaseScale))) (* (- 1.0 _alpha) 0.1))) (Variables|Default|GetBaseScale) _alpha)))))))))

(event Custom|InitializeWithId
  (params (ID :type Integer))
  ;[1 1 1] Initialize with ID
  (bind _output_get (Variables|Default|SetInteractionPitchId (Math|Integer|%(Integer) ID 12)))
  (bind _notecolor (CallFunction|GetColorbyNoteId _output_get))
  (Variables|Default|SetGlobalInteractionColor (* _notecolor 0.1)))

(event Custom|SoundDetectedEvent
  (params (mode :type Integer :default 0) (value :type Integer :default 0) (pitchId :type Integer :default 0) (volume :type Float%20%28single-precision%29)))

(event EventBeginPlay
  ;[1 1 1] Begin Play
  (bind _outactors (Actor|GetAllActorsOfClass "/Game/Blueprints/BP_Microphone_Input.BP_Microphone_Input_C"))
  (Utilities|IsValid (Utilities|Array|Get(acopy) _outactors)
    (:Is%20Valid
      (bind _output_get (Variables|Default|SetSoundComponent (Variables|/Game/Blueprints/BP_Microphone_Input.BP_Microphone_Input_C|GetSound (Utilities|Array|Get(acopy) _outactors))))
      (EventDispatchers|BindEventtoOnEventMiditoPlay _output_get (delegate Custom|MidiInteractionEvent))
      (EventDispatchers|BindEventtoOnEventWallInteraction _output_get (delegate Custom|HandleWallInteraction)))
    (:Is%20Not%20Valid
      (Development|PrintString "SIO_Floating: MicrophoneInput not valid" true true "(R=1.000000,G=0.000000,B=0.000000,A=1.000000)" 1e+01))))

(event Collision|EventActorBeginOverlap
  (params (OtherActor :type Actor%20Object%20Reference)))

(event EventHandleInputNoteId
  (params (NoteId :type Integer) (Value :type Integer))
  ;[1 1 1] Handle Input Note Id
  (if (and (Variables|Default|GetIsInInteractiveMode) (!= (Variables|Default|GetCurrentNotePlaying) NoteId))
    (switch Utilities|FlowControl|Switch|SwitchonInstrumentState (Variables|Default|GetInteractionMode)
      (:NewEnumerator0
        _)
      (:NewEnumerator1
        _))
    (bind _outactors (Actor|GetAllActorsOfClass "/Game/Blueprints/BP_MidiManager.BP_MidiManager_C"))
    (Default|StopMidiNoteonChannel (Utilities|Array|Get(acopy) _outactors) (Variables|Default|GetInstrumentChannel) (Variables|Default|GetNoteToStop))
    (bind _output_get (Variables|Default|SetCurrentNotePlaying NoteId))
    (Variables|Default|SetNoteToStop _output_get)
    (Default|PlayMidiNoteonChannel (Utilities|Array|Get(acopy) _outactors) (Variables|Default|GetInstrumentChannel) (Variables|Default|GetCurrentNotePlaying))
    (Class|SoundComponent|CallWallIneraction (Variables|Default|GetSoundComponent) true (Math|Conversions|ToInteger(Byte) (Variables|Default|GetInteractionMode)) (Variables|Default|GetCurrentNotePlaying))))

(event EventTick
  (params (DeltaSeconds :type Float%20%28single-precision%29)))

(event EventChooseInteractionMode
  (bind _instrumentchannel (Variables|Default|GetInstrumentChannel))
  (bind _instrumentchannel_2 (Variables|Default|GetInstrumentChannel))
  ;[1 1 1] Choose Interaction Mode
  (|CallParentFunction)
  (switch int (Variables|Default|GetDetectedInteractionOnsets)
    (:1
      (Class|SoundComponent|CallWallIneraction (Variables|Default|GetSoundComponent) true 0 -1)
      (bind _outactors (Actor|GetAllActorsOfClass "/Game/Blueprints/BP_MidiManager.BP_MidiManager_C"))
      (Default|HandleChannelonFirstPlace (Utilities|Array|Get(acopy) _outactors) _instrumentchannel)
      (Default|ExcludeChannelfromFileData (Utilities|Array|Get(acopy) _outactors) (Utilities|Array|MakeArray _instrumentchannel)))
    (:2
      (Class|SoundComponent|CallWallIneraction (Variables|Default|GetSoundComponent) true 1 -1)
      (bind _outactors_2 (Actor|GetAllActorsOfClass "/Game/Blueprints/BP_MidiManager.BP_MidiManager_C"))
      (Default|HandleChannelonFirstPlace (Utilities|Array|Get(acopy) _outactors_2) _instrumentchannel_2)
      (Default|ExcludeChannelfromFileData (Utilities|Array|Get(acopy) _outactors_2) (Utilities|Array|MakeArray _instrumentchannel_2)))
    (:3
      (Variables|Default|SetCanInteract false)
      (Utilities|Time|SetTimerbyFunctionName 0 "ReleaseInteraction" 1.7)
      (if (Utilities|Enum|Equal(Enum) (Variables|Default|GetInteractionMode) "NewEnumerator2")
        (Class|SoundComponent|CallWallIneraction (Variables|Default|GetSoundComponent) false 2 -1)
        (bind _outactors_3 (Actor|GetAllActorsOfClass "/Game/Blueprints/BP_MidiManager.BP_MidiManager_C"))
        (Default|IncludeChanneltoFileData (Utilities|Array|Get(acopy) _outactors_3) (Utilities|Array|MakeArray (Variables|Default|GetInstrumentChannel)))
        (else
          (Class|SoundComponent|CallWallIneraction (Variables|Default|GetSoundComponent) false 3 -1)
          (bind _outactors_4 (Actor|GetAllActorsOfClass "/Game/Blueprints/BP_MidiManager.BP_MidiManager_C"))
          (Default|ExcludeChannelfromFileData (Utilities|Array|Get(acopy) _outactors_4) (Utilities|Array|MakeArray (Variables|Default|GetInstrumentChannel)))))
      (Variables|Default|SetIsInInteractiveMode false))))

(event EventVoiceInteraction
  (params (MidiNote :type Integer) (TimeDifference :type Integer) (EventType :type Integer))
  ;[1 1 1] Midi Interaction
  (Variables|Default|SetCurrentNoteID MidiNote)
  (Variables|Default|SetCurrentTimeDifference TimeDifference)
  (Variables|Default|SetCurrentEventType EventType)
  (if (== (Variables|Default|GetCurrentEventType) (Variables|Default|GetMidiNoteOn))
    (Components|Timeline|SetPlayRate (Variables|Default|GetSmoothColorLerp) (/ 1.0 (/ (Math|Conversions|ToFloat(Integer) (Variables|Default|GetCurrentTimeDifference)) 1e+03)))
    (bind _alpha (Timeline|SmoothColorLerp PlayFromStart)
      (:Update
        (Rendering|Material|SetVectorParameterValue (Variables|Default|GetMaterial) "Color" (Math|Color|Lerp(LinearColor) (Variables|Default|GetGlobalInteractionColor) (Variables|Default|GetIdleColor) _alpha) :!class /Script/Engine.MaterialInstanceDynamic)
        (Transformation|SetWorldScale3D (Variables|Default|GetFrequency) (Math|Vector|Lerp(Vector) (- (Variables|Default|GetBaseScale) (* (Math|Vector|MakeVector 0.0 0.0 (.z (Variables|Default|GetBaseScale))) (* (- 1.0 _alpha) 0.1))) (Variables|Default|GetBaseScale) _alpha))))))

(event EventHandleInputSilence
  ;[1 1 1] Handle Input Silence
  (switch Utilities|FlowControl|Switch|SwitchonInstrumentState (Variables|Default|GetInteractionMode)
    (:NewEnumerator0
      (Class|SoundComponent|CallWallIneraction (Variables|Default|GetSoundComponent) true 0 -2))
    (:NewEnumerator1
      (Class|SoundComponent|CallWallIneraction (Variables|Default|GetSoundComponent) true 1 -2)))
  (bind _outactors (Actor|GetAllActorsOfClass "/Game/Blueprints/BP_MidiManager.BP_MidiManager_C"))
  (Default|StopMidiNoteonChannel (Utilities|Array|Get(acopy) _outactors) (Variables|Default|GetInstrumentChannel) (Variables|Default|GetNoteToStop)))

(event EventHandleInputOnset
  ;[1 1 1] Handle Input Onset
  (|CallParentFunction))

(event EventHandleOnsetChangeInteraction
  ;[1 1 1] Handle Onset Change Interaction
  (|CallParentFunction)
  (switch int (Variables|Default|GetDetectedInteractionOnsets)
    (:1
      (if (Utilities|Enum|Equal(Enum) (Variables|Default|GetInteractionMode) "NewEnumerator1")
        (CallFunction|SetInstrumentbyLastNote)))
    (:2
      (Variables|Default|SetCanInteract false)
      (Utilities|Time|SetTimerbyFunctionName 0 "ReleaseInteraction" 1.0)
      (Class|SoundComponent|CallWallIneraction (Variables|Default|GetSoundComponent) false 0 -1)
      (bind _outactors (Actor|GetAllActorsOfClass "/Game/Blueprints/BP_MidiManager.BP_MidiManager_C"))
      (Default|AllChannelsonSameLevel (Utilities|Array|Get(acopy) _outactors))
      (bind _outactors_2 (Actor|GetAllActorsOfClass "SIO_Hex_Floor_Tile_Edge_C"))
      (for _array_element _outactors_2
        (Variables|/Game/Blueprints/BP_Sound_Interactive_Object.BP_Sound_Interactive_Object_C|SetInteractionMode _array_element "NewEnumerator2")
        (Variables|/Game/Blueprints/BP_Sound_Interactive_Object.BP_Sound_Interactive_Object_C|SetIsInInteractiveMode _array_element false)
        (Default|IncludeChanneltoFileData (Utilities|Array|Get(acopy) _outactors) (Utilities|Array|MakeArray (Variables|Default|GetInstrumentChannel)))))))

(fn ConstructionScript
  (|CallParentFunction)
  (Variables|Default|SetActorLocation (Transformation|GetWorldLocation (Variables|Default|GetStaticMesh)))
  (bind _returnvalue (Rendering|Material|CreateDynamicMaterialInstance (Variables|Default|GetFrequency) 0 "/Game/Materials/Mat_Glass_Thin.Mat_Glass_Thin" :!class /Script/Engine.PrimitiveComponent))
  (Variables|Default|SetMaterial _returnvalue))