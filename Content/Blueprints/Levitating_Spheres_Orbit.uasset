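; Levitating spheres orbit Blueprint that builds a circular spline path named Orbit, with no sphere movement in its graphs.
; On BeginPlay it clears the spline and places four local-space points on the X and Y axes at SplineRadius.
; It sets perpendicular tangents scaled by the radius and a square-root-of-two constant, the Bezier-style technique for approximating a circle with four segments.
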(event EventBeginPlay
  (bind _orbit (Variables|Default|GetOrbit))
  (bind _splineradius (Variables|Default|GetSplineRadius))
  (bind _returnvalue (* _splineradius -1.0))
  (Spline|ClearSplinePoints (Variables|Default|GetOrbit) false)
  (Spline|AddSplinePoint _orbit (Math|Vector|MakeVector _splineradius 0.0 0.0) "Local" true)
  (Spline|AddSplinePoint _orbit (Math|Vector|MakeVector 0.0 _splineradius 0.0) "Local" true)
  (Spline|AddSplinePoint _orbit (Math|Vector|MakeVector _returnvalue 0.0 0.0) "Local" true)
  (Spline|AddSplinePoint _orbit (Math|Vector|MakeVector 0.0 _returnvalue 0.0) "Local" true)
  (bind _output_get (Variables|Default|SetTangentMultiplier (|(((4*((sqrt(2))-1))/3)+1))))
  (Spline|SetTangentatSplinePoint _orbit 0 (Math|Vector|MakeVector 0.0 (* _output_get (Variables|Default|GetSplineRadius) 1.0) 0.0) "Local" true)
  (Spline|SetTangentatSplinePoint _orbit 1 (Math|Vector|MakeVector (* (Variables|Default|GetTangentMultiplier) (Variables|Default|GetSplineRadius) -1.0) 0.0 0.0) "Local" true)
  (Spline|SetTangentatSplinePoint _orbit 2 (Math|Vector|MakeVector 0.0 (* (Variables|Default|GetTangentMultiplier) (Variables|Default|GetSplineRadius) -1.0) 0.0) "Local" true)
  (Spline|SetTangentatSplinePoint _orbit 3 (Math|Vector|MakeVector (* _output_get (Variables|Default|GetSplineRadius) 1.0) 0.0 0.0) "Local" true))

(event Collision|EventActorBeginOverlap
  (params (OtherActor :type Actor%20Object%20Reference)))

(event EventTick
  (params (DeltaSeconds :type Float%20%28single-precision%29)))

(fn ConstructionScript)