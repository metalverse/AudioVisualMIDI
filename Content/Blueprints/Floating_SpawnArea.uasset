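; Floating_SpawnArea is a box-shaped area that supplies random 3D spawn positions.
; Its construction script sizes the SpawnArea box from AreaExtents.
; GetNewSpawnPosition3D picks a point within those extents using a random stream, offset by the root's world location without applying rotation.
; The function ignores its Amount and ActorToSpawn inputs, as its actor-spawning loop is disconnected and never runs.
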(event EventBeginPlay)

(event Collision|EventActorBeginOverlap
  (params (OtherActor :type Actor%20Object%20Reference)))

(event EventTick
  (params (DeltaSeconds :type Float%20%28single-precision%29)))

(fn ConstructionScript
  (Components|Box|SetBoxExtent (Variables|Default|GetSpawnArea) (Variables|Default|GetAreaExtents) true))

(fn GetNewSpawnPosition3D
  (params (Amount :type Integer) (ActorToSpawn :type Actor%20Class%20Reference))
  (bind _stream (Variables|Default|GetStream))
  (bind _areaextents (Variables|Default|GetAreaExtents))
  (return (+ (Math|Vector|MakeVector (Math|Random|RandomFloatinRangefromStream (* (.x _areaextents) -1.0) (.x _areaextents) _stream) (Math|Random|RandomFloatinRangefromStream (* (.y _areaextents) -1.0) (.y _areaextents) _stream) (Math|Random|RandomFloatinRangefromStream (* (.z _areaextents) -1.0) (.z _areaextents) _stream)) (Transformation|GetWorldLocation (Variables|Default|GetDefaultSceneRoot)))))