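; Spawns a hexagon-shaped floor of hex tiles around the actor at BeginPlay, with levitating spheres at random spots.
; RandomFloatingSphereTiles first picks unique axial coordinates by retry sampling, keeping them within a scaled radius and away from the center.
; SpawnGrid then lays centered rows in two halves, converting indices to center-relative axial coordinates.
; Picked cells get an interactive tile with an attached, colored, numbered sphere below, while edge tiles spawn raised as a rim.
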(event Custom|SpawnGrid
  (bind _halfspawnsize (Variables|Default|GetHalfSpawnSize))
  (bind _halfspawnsize_2 (Variables|Default|GetHalfSpawnSize))
  (bind _tileradius (Variables|Default|GetTileRadius))
  (bind _gridpadding (Variables|Default|GetGridPadding))
  (bind _returnvalue (+ _tileradius _gridpadding))
  (Variables|Default|SetGridXOff (* (Math|Trig|Cos(Degrees) 3e+01) _returnvalue))
  (Variables|Default|SetGridYOff (* (Math|Trig|Sin(Degrees) 3e+01) _returnvalue))
  (for _index (range 0 _halfspawnsize_2)
    (bind _output_get (Variables|Default|SetColumns (+ _index _halfspawnsize_2)))
    (for _index_2 (range 0 _output_get)
      (bind _xposition (CallFunction|CalculateXPosition _index_2))
      (bind _yposition (CallFunction|CalculateYPosition -1))
      (CallFunction|SpawnGridTileatPoint (Math|Vector|MakeVector _xposition _yposition (.z (Variables|Default|GetCenterPoint))) _index_2 _index)))
  (for _index_3 (range (Variables|Default|GetHalfSpawnSize) (Variables|Default|GetSpawnSize))
    (bind _output_get_2 (Variables|Default|SetColumns (+ (- (Variables|Default|GetSpawnSize) _index_3) _halfspawnsize)))
    (for _index_4 (range 0 _output_get_2)
      (bind _xposition_2 (CallFunction|CalculateXPosition _index_4))
      (bind _yposition_2 (CallFunction|CalculateYPosition 1))
      (CallFunction|SpawnGridTileatPoint (Math|Vector|MakeVector _xposition_2 _yposition_2 (.z (Variables|Default|GetCenterPoint))) (+ _index_4 (- _index_3 _halfspawnsize)) _index_3))))

(event EventBeginPlay
  (bind _returnvalue (Transformation|GetActorLocation))
  (Variables|Default|SetCenterPoint (Math|Vector|MakeVector (- (.x _returnvalue) 8e+01) (.y _returnvalue) (.z _returnvalue)))
  (Variables|Default|SetHalfSpawnSize (/ (Variables|Default|GetSpawnSize) 2))
  (CallFunction|RandomFloatingSphereTiles)
  (CallFunction|SpawnGrid))

(event Collision|EventActorBeginOverlap
  (params (OtherActor :type Actor%20Object%20Reference)))

(event EventTick
  (params (DeltaSeconds :type Float%20%28single-precision%29)))

(fn ConstructionScript)

(fn SpawnGridTileatPoint
  (params (SpawnPosition :type Vector) (Column :type Integer) (Row :type Integer))
  (bind _halfspawnsize (Variables|Default|GetHalfSpawnSize))
  (bind _spawnedlevitatingspheres (Variables|Default|GetSpawnedLevitatingSpheres))
  (bind _returnvalue (- Row _halfspawnsize))
  (bind _output_get (LocalVariables|SetTileColumn (- (- Column _halfspawnsize) _returnvalue)))
  (bind _output_get_2 (LocalVariables|SetTileRow _returnvalue))
  (if (Utilities|Array|ContainsItem (Variables|Default|GetFloatingPositionTiles) (Math|Vector2D|MakeVector2D (Math|Conversions|ToFloat(Integer) _output_get_2) (Math|Conversions|ToFloat(Integer) _output_get)))
    (bind _returnvalue_2 (Game|SpawnActorfromClass "/Game/Blueprints/SIO_Levitating_Sphere.SIO_Levitating_Sphere_C" (Math|Transform|MakeTransform (+ SpawnPosition "0, 0,-60.000000") "0, 0,0.000000" "1.000000,1.000000,1.000000") "Undefined" 0 (Utilities|Array|Get(acopy) (Variables|Default|GetBaseColorsInCircle) _spawnedlevitatingspheres) _spawnedlevitatingspheres))
    (bind _returnvalue_3 (Game|SpawnActorfromClass "/Game/Blueprints/SIO_Hex_Floor_Tile_Interactive.SIO_Hex_Floor_Tile_Interactive_C" (Math|Transform|MakeTransform SpawnPosition "0, 0,0.000000" "1.000000,1.000000,1.000000") "Undefined" 0 0))
    (Transformation|AttachActorToActor _returnvalue_2 _returnvalue_3 "None" "KeepWorld" "KeepWorld" "KeepWorld" true)
    (Math|Integer|IncrementInt (Variables|Default|GetSpawnedLevitatingSpheres)
      (:%20%20
        _))
    (else
      (bind _isedgetile (CallFunction|IsEdgeTile (LocalVariables|GetTileRow) (LocalVariables|GetTileColumn)))
      (if _isedgetile
        (bind _returnvalue_4 (Game|SpawnActorfromClass "/Game/Blueprints/SIO_Hex_Floor_Tile.SIO_Hex_Floor_Tile_C" (Math|Transform|MakeTransform (+ SpawnPosition "0, 0,150.000000") "0, 0,0.000000" "1.000000,1.000000,1.000000") "Undefined" 0 (LocalVariables|GetTileRow) (LocalVariables|GetTileColumn)))
        (else
          (Game|SpawnActorfromClass "/Game/Blueprints/SIO_Hex_Floor_Tile.SIO_Hex_Floor_Tile_C" (Math|Transform|MakeTransform SpawnPosition "0, 0,0.000000" "1.000000,1.000000,1.000000") "Undefined" 0 (LocalVariables|GetTileRow) (LocalVariables|GetTileColumn))))))
  (Math|Integer|IncrementInt (Variables|Default|GetSpawnedTiles)))

(fn CalculateXPosition
  (params (Column :type Integer))
  (return (+ (* (+ (+ (* Column 2) 1) (* (Variables|Default|GetColumns) -1)) (Variables|Default|GetGridXOff)) (.x (Variables|Default|GetCenterPoint)))))

(fn CalculateYPosition
  (params (Factor :type Integer))
  (return (+ (* (* (- (Variables|Default|GetSpawnSize) (Variables|Default|GetColumns)) 3) (* Factor (Variables|Default|GetGridYOff))) (.y (Variables|Default|GetCenterPoint)))))

(fn RandomFloatingSphereTiles
  (bind _output_get (LocalVariables|SetTreshold (Math|Float|Truncate (* (Variables|Default|GetHalfSpawnSize) (Variables|Default|GetSpheresRangeMultiplier)))))
  (for _index (range 0 (- (Variables|Default|GetLevitatingSpheresToSpawn) 1))
    (bind _output_get_2 (LocalVariables|SetXValue (Math|Random|RandomIntegerinRange (* _output_get -1) _output_get) :!label _label))
    (if (> _output_get_2 0)
      (LocalVariables|SetYValue (Math|Random|RandomIntegerinRange (* (LocalVariables|GetTreshold) -1) (Math|Float|Truncate (* _output_get_2 (Variables|Default|GetSpheresRangeMultiplier)))))
      (else
        (LocalVariables|SetYValue (Math|Random|RandomIntegerinRange (- (* (LocalVariables|GetTreshold) -1) _output_get_2) (LocalVariables|GetTreshold)))))
    (if (or (> (+ (LocalVariables|GetXValue) (LocalVariables|GetYValue)) (LocalVariables|GetTreshold)) (< (+ (Math|Integer|Absolute(Integer) (LocalVariables|GetXValue)) (Math|Integer|Absolute(Integer) (LocalVariables|GetYValue))) 3))
      (goto _label)
      (else
        (bind _returnvalue (Utilities|Array|AddUnique (Variables|Default|GetFloatingPositionTiles) (Math|Vector2D|MakeVector2D (Math|Conversions|ToFloat(Integer) (LocalVariables|GetXValue)) (Math|Conversions|ToFloat(Integer) (LocalVariables|GetYValue)))))
        (if (not (== _returnvalue _index))
          (goto _label))))))

(fn IsEdgeTile
  (params (Row :type Integer) (Column :type Integer))
  (bind _halfspawnsize (Variables|Default|GetHalfSpawnSize))
  (if (or (== (Math|Integer|Absolute(Integer) Row) _halfspawnsize) (== (Math|Integer|Absolute(Integer) Column) _halfspawnsize))
    _
    (elif (== (Math|Integer|Absolute(Integer) (+ Row Column)) (Variables|Default|GetHalfSpawnSize))
      _
      (else
        (return false))))
  (return true))