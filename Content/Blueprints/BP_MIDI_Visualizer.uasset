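; MIDI player and visualizer that plays the game instance's level track, with loop, tempo and per-channel toggle controls.
; On BeginPlay it spawns the keyboard, ball, statues, dust and floating objects.
; Filtered MIDI events go to the synth output and animate those props, spheres and percussion antennas by channel, while ticks fire Beat events.
; Tick sends pan messages computed from player position and facing relative to the world origin.
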(event OnEventTempo(Midi)
  (params (mpqn :type Integer) (ppq :type Integer))
  ;[1 1 1] Tempo Event
  (bind _output_get (Variables|Midi|SetMidiMPQN mpqn))
  (bind _output_get_2 (Variables|Midi|SetMidiPPQ ppq))
  (Variables|Midi|SetMidiTempoBpm (/ 60000000 _output_get))
  (CallFunction|SetBeatTicksTreshold _output_get_2)
  (Development|PrintString (Utilities|String|Append "New MPQN " (Utilities|String|ToString(Integer) _output_get) "| PPQ " (Utilities|String|ToString(Integer) _output_get_2)) true true "(R=0.000000,G=0.660000,B=1.000000,A=1.000000)" 1e+01))

(event OnSend(Midi)
  (params (msg :type Array%20of%20Bytes) (elapsed :type Integer) (channel :type Integer) (midiEventType :type Integer))
  ;[1 1 1] Device Midi Synth
  (bind _playnote (CallFunction|ShouldNotebePlayed channel midiEventType))
  (if _playnote
    (Class|MidiInterface|SendMidiMessage msg)
    (CallFunction|PrintMidiMessage msg)))

(event OnEventTicks(Midi)
  (params (ticksElapsed :type Integer))
  ;[1 1 1] Ticks Event
  (Utilities|FlowControl|Sequence
    (:then_0
      (if (< ticksElapsed (Variables|Default|GetLastTicksElapsed))
        (Variables|Midi|SetTicksElapsed (- (Variables|Midi|GetTicksElapsed) (Variables|Default|GetLastTicksElapsed)))
        (Variables|Default|SetLastTicksElapsed 0))
      (if (> (- ticksElapsed (Variables|Default|GetLastTicksElapsed)) (Variables|Default|GetTicksForBeatStepTreshold))
        (bind _output_get (Variables|Default|SetLastTicksElapsed (+ (Variables|Default|GetLastTicksElapsed) (Variables|Default|GetTicksForBeatStep))))
        (Variables|Default|SetLastTicksElapsed (+ (Variables|Default|GetLastTicksElapsed) (Variables|Default|GetTicksForBeatStep)))
        (Class|BeatComponent|CallBeatEvent (Variables|Default|GetBeat))))))

(event OnEventwithInfo(Midi)
  (params (track :type Integer) (note :type Integer) (velocity :type Integer) (nextNote :type Integer) (timeDifference :type Integer) (eventType :type Integer) (elapsed :type Integer))
  ;[1 1 1] Processing Visual Events
  ;;[0.1203 0 1] Processed Events
  (bind _playnote (CallFunction|ShouldNotebeVisualized track eventType))
  (if _playnote
    (Variables|Midi|SetCurrentNoteVelocity velocity)
    (Variables|Midi|SetCurrentNote note)
    (Variables|Midi|SetChannel track)
    (Variables|Midi|SetNextNote nextNote)
    (Variables|Midi|SetTimeDifference timeDifference)
    (Variables|Midi|SetMidiEventType eventType)
    (if (and (== (Variables|Midi|GetChannel) 0) (== (Variables|Midi|GetMidiEventType) (Variables|Midi|GetMidiNoteOn)))
      (Default|UpdatePosition (Variables|Instruments|GetBall) (Variables|Midi|GetNextNote) (Variables|Midi|GetTimeDifference)))
    (Default|Update (Variables|Instruments|GetMidiKeyboard) (Variables|Midi|GetChannel) (Variables|Midi|GetCurrentNote) (Variables|Midi|GetNextNote) (Variables|Midi|GetTimeDifference) (Variables|Midi|GetMidiEventType))
    (if (not (== (Variables|Midi|GetChannel) 8))
      (if (== (Variables|Midi|GetChannel) 9)
        (Default|MidiInteraction (Variables|Instruments|GetPercussionAntenas))
        (elif (== (Variables|Midi|GetChannel) 4)
          (for _array_element (Variables|Instruments|GetVisualStatues)
            (Rendering|Material|SetVectorParameterValue _array_element "Color" (Math|Color|SelectColor (Utilities|Array|Get(acopy) (Variables|Instruments|GetVisualCubesColors) (Variables|Midi|GetChannel)) "(R=0.000000,G=0.000000,B=0.000000,A=1.000000)" (== (Variables|Midi|GetMidiEventType) (Variables|Midi|GetMidiNoteOn))) :!class /Script/Engine.MaterialInstanceDynamic))
          (elif (== (Variables|Midi|GetChannel) 1)
            (for _array_element_2 (Variables|Instruments|GetLevitatingSpheres)
              (Default|MidiInteraction _array_element_2 (Variables|Midi|GetCurrentNote) 0 (Variables|Midi|GetTimeDifference) (Variables|Midi|GetMidiEventType)))
            (Default|MidiInteraction (Variables|Instruments|GetBassSphere) (Variables|Midi|GetCurrentNote) 0 (Variables|Midi|GetTimeDifference) (Variables|Midi|GetMidiEventType))))))))

(event OnEvent(Midi)
  (params (track :type Integer) (note :type Integer) (velocity :type Integer) (elapsed :type Integer)))

(event Custom|PlayTrack
  (bind _midi (Variables|Default|GetMidi))
  ;[1 1 1] Play Track
  (Class|MidiComponent|LoadAsset _midi (Variables|Default|GetMidi%20Asset))
  (Class|MidiComponent|Start _midi)
  (Default|CallOnChangeSunPosition 0.0))

(event Custom|PlayTrackLooped
  (bind _midi (Variables|Default|GetMidi))
  (Class|MidiComponent|LoadAsset _midi (Variables|Default|GetMidi%20Asset))
  (Class|MidiComponent|StartwithLoop _midi 1 2))

(event Custom|SetLevitatingSpheresReferences
  (bind _outactors (Actor|GetAllActorsOfClass "/Game/Blueprints/SIO_Levitating_Sphere.SIO_Levitating_Sphere_C"))
  (for _array_element _outactors
    (Utilities|Array|Add (Variables|Instruments|GetLevitatingSpheres) _array_element))
  (bind _outactors_2 (Actor|GetAllActorsOfClass "/Game/Blueprints/SIO_Bass_Sphere.SIO_Bass_Sphere_C"))
  (Variables|Instruments|SetBassSphere (Utilities|Array|Get(acopy) _outactors_2)))

(event Custom|ChangeMIDITempoRealTime
  (params (NewBPM :type Float%20%28single-precision%29))
  (bind _miditempobpm (Variables|Midi|GetMidiTempoBpm))
  (bind _midi (Variables|Default|GetMidi))
  (bind _returnvalue (Math|Conversions|ToFloat(Integer) _miditempobpm))
  (bind _returnvalue_2 (/ NewBPM _returnvalue))
  ;[1 1 1] Real Time change MIDI tempo
  (if (Class|MidiComponent|IsRunning _midi)
    (bind _alpha (Timeline|Timeline_0 PlayFromStart)
      (:Update
        (Class|MidiComponent|SetTempoMultiplier _midi (Math|Float|Lerp (Variables|Midi|GetCurrentTempoMultiplier) _returnvalue_2 _alpha)))
      (:Finished
        (Variables|Midi|SetCurrentTempoMultiplier _returnvalue_2)))))

(event Custom|MidiStopped
  (params (finished :type Boolean))
  ;[1 1 1] Device Midi Synth
  (Development|PrintString "Stop")
  (CallFunction|StopVizualize))

(event Custom|StopTrack
  ;[1 1 1] Stop Track
  (Class|MidiComponent|Stop (Variables|Default|GetMidi))
  (CallFunction|StopVizualize)
  (Default|CallOnChangeSunPosition -5.0))

(event Custom|ChangeMIDITempo
  (params (NewBPM :type Float%20%28single-precision%29))
  (bind _midi (Variables|Default|GetMidi))
  (bind _miditempobpm (Variables|Midi|GetMidiTempoBpm))
  (bind _returnvalue (Math|Conversions|ToFloat(Integer) _miditempobpm))
  (bind _returnvalue_2 (/ NewBPM _returnvalue))
  ;[1 1 1] Change MIDI tempo
  (if (Class|MidiComponent|IsRunning _midi)
    (Class|MidiComponent|SetTempoMultiplier _midi _returnvalue_2)
    (bind _output_get (Variables|Midi|SetCurrentTempoMultiplier _returnvalue_2))))

(event Custom|ChangeLoopRange
  (params (StartBar :type Integer) (EndBar :type Integer))
  (Class|MidiComponent|SetLoopRange (Variables|Default|GetMidi) StartBar EndBar))

(event EventEndPlay
  (params (EndPlayReason :type EEndPlayReason%20Enum :default "Destroyed"))
  ;[1 1 1] Device Midi Synth
  (Class|MidiInterface|CloseMidiOutput)
  (CallFunction|StopVizualize))

(event EventBeginPlay
  ;[0 1 0.6045] Setup Midi
  (|CallParentFunction)
  (EventDispatchers|BindEventtoOnStop (Variables|Default|GetMidi) (delegate Custom|MidiStopped))
  ;[1 1 1] Create Visual Cubes
  (Utilities|FlowControl|Sequence
    (:then_0
      (bind _asmy_game_instance (Utilities|Casting|CastToMyGameInstance (Game|GetGameInstance (Game|Player|GetPlayerPawn 0))))
      (Variables|Default|SetMidi%20Asset (Variables|/Game/GameInstances/MyGameInstance.MyGameInstance_C|GetLevelMidiAsset _asmy_game_instance)))
    (:then_1
      (bind _returnvalue (Game|SpawnActorfromClass "/Game/Blueprints/VisualBoxes.VisualBoxes_C" (Math|Transform|MakeTransform "800.000000,-287.000000,70.000000" "0, 0, 0" "1,1,1") "Undefined" 0 0))
      (Variables|Instruments|SetMidiKeyboard _returnvalue)
      (for _index (range 0 20)
        (Utilities|Array|Add (Variables|Instruments|GetVisualCubesColors) (Utilities|Struct|MakeLinearColor (Math|Random|RandomFloat) (Math|Random|RandomFloat) (Math|Random|RandomFloat) 1.0)))
      (CallFunction|SpawnVisualStatue "777.000000,-1350.000000, 0")
      (CallFunction|SpawnVisualStatue "777.000000,1350.000000, 0")
      (CallFunction|SpawnVisualStatue "-780.000000,1350.000000, 0")
      (CallFunction|SpawnVisualStatue "-1560.000000,0.000000, 0")
      (CallFunction|SpawnVisualStatue "-780.000000,-1350.000000, 0")
      (bind _returnvalue_2 (Game|SpawnActorfromClass "/Game/Blueprints/DustDrops.DustDrops_C" (Math|Transform|MakeTransform (Math|Vector|MakeVector -1e+03 -2e+02 4e+02) "-40.000000,25.000000, 0" "1,1,1") "Undefined" 0 0))
      (Variables|Default|SetDust _returnvalue_2)
      (bind _returnvalue_3 (Game|SpawnActorfromClass "/Game/Blueprints/Midi_Ball.Midi_Ball_C" (Math|Transform|MakeTransform (+ (Variables|Default|GetStartLocation) "1600.000000, 0,230.000000") "0, 0, 0" "1,1,1") "Undefined" 0 0))
      (Variables|Instruments|SetBall _returnvalue_3)
      (CallFunction|SpawnFloatingObjects (Variables|Default|GetFloatingObjectsAmount)))
    (:then_2
      (bind _outactors (Actor|GetAllActorsOfClass "/Game/Blueprints/SIO_Percussion_Antenas.SIO_Percussion_Antenas_C"))
      (Utilities|IsValid (Utilities|Array|Get(acopy) _outactors)
        (:Is%20Valid
          (Variables|Instruments|SetPercussionAntenas (Utilities|Array|Get(acopy) _outactors)))))))

(event EventTick
  (params (DeltaSeconds :type Float%20%28single-precision%29))
  ;[1 1 1] Event Tick
  (if (Class|MidiComponent|IsRunning (Variables|Default|GetMidi))
    (Variables|Default|SetTicksElapsedForPanorama (+ DeltaSeconds (Variables|Default|GetTicksElapsedForPanorama)))
    (if (> (Variables|Default|GetTicksElapsedForPanorama) 0.1)
      (CallFunction|HandleActiveIntrumentsPanorama)
      (Variables|Default|SetTicksElapsedForPanorama 0.0))))

(fn ConstructionScript)

(fn SpawnEmitter
  (params (Note :type Integer))
  (bind _emitter (Variables|Default|GetEmitter))
  (Utilities|IsValid _emitter
    (:Is%20Valid
      (Actor|DestroyActor _emitter))
    (:Is%20Not%20Valid
      _))
  (LocalVariables|SetHeight (+ (* (Math|Conversions|ToFloat(Integer) Note) 7.0) 8e+01))
  (bind _returnvalue (Game|SpawnActorfromClass "/Game/ElectricityArc_BP.ElectricityArc_BP_C" (Math|Transform|MakeTransform (Math|Vector|MakeVector 0.0 -6.5e+02 (LocalVariables|GetHeight)) "0, 0, 0" "1,1,1") "AlwaysSpawn" 0 0))
  (Class|ParticleSystemComponent|SetBeamTargetPoint (Variables|/Game/ElectricityArc_BP.ElectricityArc_BP_C|GetEmitter _returnvalue) 0 (Math|Vector|MakeVector 0.0 6.5e+02 (LocalVariables|GetHeight)))
  (return _returnvalue))

(fn SpawnRain
  (for _index (range 0 3)
    (Game|SpawnActorfromClass "/Game/Blueprints/WaterDrops.WaterDrops_C" (Math|Transform|MakeTransform (Math|Vector|MakeVector -5e+02 (+ (* _index 3e+02) -6e+02) 8e+02) "0, 0, 0" "1,1,1") "Undefined" 0 0))
  (Actor|DestroyActor (Variables|Default|GetDust)))

(fn ShouldNotebePlayed
  (params (ChannelNumber :type Integer) (EventType :type Integer))
  (return (or (Utilities|Array|ContainsItem (Variables|Midi|GetChannelsToPlay) ChannelNumber) (== EventType (LocalVariables|GetNoteOffEventType)))))

(fn AddChanneltoPlay
  (params (ChannelToAdd :type Integer))
  (Utilities|Array|AddUnique (Variables|Midi|GetChannelsToPlay) ChannelToAdd)
  (CallFunction|AddChanneltoVisualize ChannelToAdd))

(fn RemoveChanneltoPlay
  (params (RemoveChannel :type Integer))
  (Utilities|Array|RemoveItem (Variables|Midi|GetChannelsToPlay) RemoveChannel)
  (CallFunction|RemoveChanneltoVisualize RemoveChannel))

(fn SwitchChanneltoPlay
  (params (Channel :type Integer))
  (if (Utilities|Array|ContainsItem (Variables|Midi|GetChannelsToPlay) Channel)
    (CallFunction|RemoveChanneltoPlay Channel)
    (else
      (CallFunction|AddChanneltoPlay Channel))))

(fn ShouldNotebeVisualized
  (params (Channel :type Integer) (EventType :type Integer))
  (return (or (Utilities|Array|ContainsItem (Variables|Midi|GetChannelsToVisualize) Channel) (== EventType (LocalVariables|GetNoteOffEventType)))))

(fn AddChanneltoVisualize
  (params (Channel :type Integer))
  (Utilities|Array|AddUnique (Variables|Midi|GetChannelsToVisualize) Channel))

(fn RemoveChanneltoVisualize
  (params (Channel :type Integer))
  (Utilities|Array|RemoveItem (Variables|Midi|GetChannelsToVisualize) Channel))

(fn SpawnFloatingObjects
  (params (Amount :type Integer))
  (bind _outactors (Actor|GetAllActorsOfClass "/Game/Blueprints/Floating_SpawnArea.Floating_SpawnArea_C"))
  (for _array_element _outactors
    (Utilities|IsValid _array_element
      (:Is%20Valid
        (for _index (range 1 Amount)
          (bind _position (Default|GetNewSpawnPosition3D _array_element 0 "/Game/Blueprints/SIO_Floating.SIO_Floating_C"))
          (Game|SpawnActorfromClass "/Game/Blueprints/SIO_Floating.SIO_Floating_C" (Math|Transform|MakeTransform (Transformation|GetActorLocation _array_element) "90.000000, 0, 0" "1,1,1") "Undefined" 0 _position 25 (Variables|Default|GetBeat)))))))

(fn SetBeatTicksTreshold
  (params (PPQ :type Integer))
  (Variables|Default|SetTicksForBeatStep PPQ)
  (bind _output_get (Variables|Default|SetTicksForBeatStepTreshold (Math|Float|Truncate (* (Variables|Default|GetTicksForBeatStep) 2.05))))
  (Development|PrintString (Utilities|String|ToString(Integer) _output_get)))

(fn StopVizualize
  (Default|TurnOffAll (Variables|Instruments|GetMidiKeyboard))
  (Variables|Midi|SetTicksElapsed 0)
  (Variables|Default|SetLastTicksElapsed 0))

(fn SpawnVisualStatue
  (params (Location :type Vector))
  (bind _returnvalue (Game|SpawnActorfromClass "/Game/Statue_BP.Statue_BP_C" (Math|Transform|MakeTransform Location "0, 0, 0" "1,1,1") "AdjustIfPossibleButAlwaysSpawn" 0 0))
  (bind _returnvalue_2 (Rendering|Material|CreateDynamicMaterialInstance (Variables|/Game/Statue_BP.Statue_BP_C|GetStaticMesh _returnvalue) 0 "/Game/Materials/MatTest.MatTest" :!class /Script/Engine.PrimitiveComponent))
  (Utilities|Array|Add (Variables|Instruments|GetVisualStatues) _returnvalue_2))

(fn ChangeTrackPanorama
  (params (Channel :type Integer) (PanValue :type Integer))
  (Class|MidiInterface|SendMidiMessage (Utilities|Array|MakeArray (+ (Math|Conversions|ToByte(Integer) Channel) 176) 10 (Math|Conversions|ToByte(Integer) PanValue))))

(fn PrintMidiMessage
  (params (Message :type Array%20of%20Bytes))
  (for _array_element Message
    (LocalVariables|SetTextMessage (Utilities|String|Append (LocalVariables|GetTextMessage) "|" (Utilities|String|ToString(Byte) _array_element))))
  (Development|PrintString (LocalVariables|GetTextMessage)))

(fn HandleActiveIntrumentsPanorama
  (bind _returnvalue (Game|GetPlayerCharacter 0))
  (bind _returnvalue_2 (Transformation|GetActorLocation _returnvalue))
  (bind _capsulecomponent (Variables|/Script/Engine.Character|GetCapsuleComponent _returnvalue))
  (bind _returnvalue_3 (Math|Vector|GetForwardVector _capsulecomponent))
  (for _array_element (Variables|Midi|GetChannelsToPlay)
    (bind _panorama (CallFunction|CalculatePanorama (Math|Vector|MakeVector (.x _returnvalue_2) (.y _returnvalue_2) 0.0) "0,0.000000, 0" (Math|Vector|MakeVector (.x _returnvalue_3) (.y _returnvalue_3) 0.0)))
    (CallFunction|ChangeTrackPanorama _array_element _panorama)))

(fn CalculatePanorama
  (params (PlayerPosition :type Vector) (InstrumentPosition :type Vector) (PlayerForward :type Vector))
  (bind (_x _y) (Math|Vector|BreakVector PlayerForward))
  (bind _returnvalue (- InstrumentPosition PlayerPosition))
  (bind (_x_2 _y_2) (Math|Vector|BreakVector _returnvalue))
  (return (Math|Float|Truncate (Math|Float|Clamp(Float) (+ (* (Math|Trig|Cos(Degrees) (Class|KismetMathLibrary|DegAtan2 (+ (Math|Vector|DotProduct _returnvalue PlayerForward) 9e+01) (- (* _y_2 _x) (* _x_2 _y)))) 64.0) 64.0) 5.0 122.0))))