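; BP_MicrophoneInput_Plus turns microphone silence state into sound events for the game.
; Each Tick it compares IsSilence with a stored WasSilence flag, so it reacts only when the state flips.
; A flip to sound prints a debug message and calls CallSoundEvent on Sound in SoundOn mode with the current Volume.
; A flip to silence only prints a message.
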(event EventBeginPlay)

(event Collision|EventActorBeginOverlap
  (params (OtherActor :type Actor%20Object%20Reference)))

(event EventTick
  (params (DeltaSeconds :type Float%20%28single-precision%29))
  (if (Variables|Default|GetisSilence)
    (if (not (Variables|Default|GetWasSilence))
      (Variables|Default|SetWasSilence true)
      (Development|PrintString "Silence"))
    (elif (Variables|Default|GetWasSilence)
      (Variables|Default|SetWasSilence false)
      (Development|PrintString "Sound!")
      (Class|SoundComponent|CallSoundEvent (Variables|Default|GetSound) (.soundon (Variables|Default|GetSoundEventModes)) 0 0 (Variables|Default|Getvolume)))))

(fn ConstructionScript)