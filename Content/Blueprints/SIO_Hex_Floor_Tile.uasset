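; SIO hex floor tile actor that lights up in response to player microphone sound, as a ripple spreading out from the player.
; It binds to the BP_MicrophoneInput_Plus sound event and creates a dynamic material on its static mesh.
; Tiles within range react when normalized volume exceeds normalized player distance, with timer delays proportional to that distance.
; Sound on sets the interaction color, sound off fades to idle through a timeline, and volume events trigger short pulses.
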(event Custom|ReactOnSoundOn
  ;[1 1 1] React On Sound
  (Variables|Default|SetIsInSoundMode true)
  (Rendering|Material|SetVectorParameterValue (Variables|Default|GetMaterial) "Color" (Variables|Default|GetGlobalInteractionColor) :!class /Script/Engine.MaterialInstanceDynamic))

(event Custom|SoundDetectedEvent
  (params (mode :type Integer) (value :type Integer) (pitchId :type Integer) (volume :type Float%20%28single-precision%29))
  (bind _soundeventmodes (Variables|Default|GetSoundEventModes))
  ;[1 1 1] Sound Detected Event
  (if (== mode (.soundon _soundeventmodes))
    (bind (_shouldreact _timeforreaction) (CallFunction|ShouldReactonSound volume))
    (if _shouldreact
      (Variables|Default|SetIsInSoundMode true)
      (Utilities|Time|SetTimerbyEvent (delegate Custom|ReactOnSoundOn) _timeforreaction))
    (elif (== mode (.soundoff _soundeventmodes))
      (if (Variables|Default|GetIsInSoundMode)
        (bind _reactdelay (CallFunction|GetReactDelay))
        (Utilities|Time|SetTimerbyEvent (delegate Custom|ReactOnSoundOff) _reactdelay))
      (elif (== mode (.volumeevent _soundeventmodes))
        (if (not (Variables|Default|GetIsInSoundMode))
          (bind (_shouldreact_2 _timeforreaction_2) (CallFunction|ShouldReactonSound volume))
          (if _shouldreact_2
            (Variables|Default|SetIsInSoundMode true)
            (Utilities|Time|SetTimerbyEvent (delegate Custom|ReactOnSoundOn) _timeforreaction_2)
            (Utilities|Time|SetTimerbyEvent (delegate Custom|ReactOnSoundOff) (+ _timeforreaction_2 0.3))))))))

(event Custom|ReactOnSoundOff
  ;[1 1 1] React On Sound Off
  (Variables|Default|SetIsInSoundMode false)
  (bind _alpha (Timeline|Timeline_0 PlayFromStart)
    (:Update
      (Rendering|Material|SetVectorParameterValue (Variables|Default|GetMaterial) "Color" (Math|Color|Lerp(LinearColor) (Variables|Default|GetGlobalInteractionColor) (Variables|Default|GetIdleColor) _alpha) :!class /Script/Engine.MaterialInstanceDynamic))))

(event EventBeginPlay
  ;[1 1 1] Begin Play
  (bind _outactors (Actor|GetAllActorsOfClass "/Game/Blueprints/BP_MicrophoneInput_Plus.BP_MicrophoneInput_Plus_C"))
  (Utilities|IsValid (Utilities|Array|Get(acopy) _outactors)
    (:Is%20Valid
      (bind _output_get (Variables|Default|SetSoundComponent (Variables|/Game/Blueprints/BP_MicrophoneInput_Plus.BP_MicrophoneInput_Plus_C|GetSound (Utilities|Array|Get(acopy) _outactors))))
      (EventDispatchers|BindEventtoOnEventSoundDetected _output_get (delegate Custom|SoundDetectedEvent))
      (Variables|Default|SetActorLocation (Transformation|GetWorldLocation (Variables|Default|GetStaticMesh)))
      (bind _returnvalue (Rendering|Material|CreateDynamicMaterialInstance (Variables|Default|GetStaticMesh) 2 "/Game/Materials/LevitatingSphere/LevitatingSphere_Inactive.LevitatingSphere_Inactive" :!class /Script/Engine.PrimitiveComponent))
      (Variables|Default|SetMaterial _returnvalue))
    (:Is%20Not%20Valid
      (Development|PrintString "SIO_Floating: MicrophoneInput not valid" true true "(R=1.000000,G=0.000000,B=0.000000,A=1.000000)" 1e+01))))

(event Collision|EventActorBeginOverlap
  (params (OtherActor :type Actor%20Object%20Reference)))

(event EventTick
  (params (DeltaSeconds :type Float%20%28single-precision%29)))

(fn ConstructionScript)

(fn ShouldReactonSound
  (params (Volume :type Float%20%28single-precision%29))
  (bind _returnvalue (Game|Player|GetPlayerPawn 0))
  (bind _maxinteractiondistance (Variables|Default|GetMaxInteractionDistance))
  (bind _actorlocation (Variables|Default|GetActorLocation))
  (bind _returnvalue_2 (Transformation|GetActorLocation _returnvalue))
  (bind _returnvalue_3 (- _returnvalue_2 _actorlocation))
  (bind _returnvalue_4 (Math|Vector|VectorLength _returnvalue_3))
  (if (< _returnvalue_4 _maxinteractiondistance)
    (if (> (Math|Float|Clamp(Float) (Math|Float|NormalizetoRange Volume 4.0 (Variables|Default|GetMaxDistanceVolume))) (Math|Float|Clamp(Float) (Math|Float|NormalizetoRange _returnvalue_4 0.0 _maxinteractiondistance)))
      (return true (/ _returnvalue_4 (Variables|Default|GetDelayDistanceDevider)))
      (else
        _)))
  (return false 0.0))

(fn GetReactDelay
  (return (/ (Math|Vector|VectorLength (- (Transformation|GetActorLocation (Game|Player|GetPlayerPawn 0)) (Variables|Default|GetActorLocation))) (Variables|Default|GetDelayDistanceDevider))))