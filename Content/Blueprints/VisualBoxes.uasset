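; VisualBoxes is a MIDI note visualizer that lights a row of thin, tall meshes, one per note number.
; BeginPlay spawns the meshes along Y, gives each a dynamic material instance and builds a random color palette indexed by channel.
; Update indexes the materials by MidiNote and sets Color to the channel's color, or black for event type 8, ignoring channels 4 and 8.
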(event Custom|Update
  (params (Channel :type Integer) (MidiNote :type Integer) (NextMidiNote :type Integer) (TimeDifference :type Integer) (EventType :type Integer))
  (if (and (!= Channel 4) (!= Channel 8))
    (Rendering|Material|SetVectorParameterValue (Utilities|Array|Get(acopy) (Variables|Default|GetVisualCubesMaterials) MidiNote) "Color" (Math|Color|SelectColor (Utilities|Array|Get(acopy) (Variables|Default|GetVisualCubesColors) Channel) "(R=0.000000,G=0.000000,B=0.000000,A=1.000000)" (!= EventType 8)) :!class /Script/Engine.MaterialInstanceDynamic)))

(event EventBeginPlay
  (bind _defaultsceneroot (Variables|Default|GetDefaultSceneRoot))
  (bind _relativelocation (Variables|/Script/Engine.SceneComponent|GetRelativeLocation _defaultsceneroot))
  (for _index (range 0 115)
    (bind _returnvalue (AddComponent|AddStaticMeshComponent false (Math|Transform|MakeTransform (Math|Vector|MakeVector (.x _relativelocation) (+ (* _index 1e+01) (.y _relativelocation)) (.z _relativelocation)) "0, 0, 0" "0.050000,0.050000,1.500000")))
    (bind _returnvalue_2 (Rendering|Material|CreateDynamicMaterialInstance _returnvalue 0 "/Game/Midi/Other/MatTest.MatTest" :!class /Script/Engine.PrimitiveComponent))
    (Utilities|Array|Add (Variables|Default|GetVisualCubesMaterials) _returnvalue_2))
  (for _index_2 (range 0 20)
    (Utilities|Array|Add (Variables|Default|GetVisualCubesColors) (Utilities|Struct|MakeLinearColor (Math|Random|RandomFloat) (Math|Random|RandomFloat) (Math|Random|RandomFloat) 1.0))))

(event Collision|EventActorBeginOverlap
  (params (OtherActor :type Actor%20Object%20Reference)))

(event EventTick
  (params (DeltaSeconds :type Float%20%28single-precision%29)))

(fn ConstructionScript)