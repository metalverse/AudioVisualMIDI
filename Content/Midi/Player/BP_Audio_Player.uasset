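; Audio player Blueprint that turns incoming MIDI note events into generated constant tones played as 2D sounds, supporting several notes at once.
; Each non-zero velocity event spawns a tone at the note's frequency with fixed amplitude and records it by track and note.
; Every event first stops and removes any matching tracked sound, so zero velocity acts as note-off and repeated notes retrigger.
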(event OnEvent(Midi)
  (params (track :type Integer) (note :type Integer) (velocity :type Integer) (elapsed :type Integer))
  (bind _2d_sound_items (Variables|Default|Get2D%20Sound%20Items))
  ;[0.1203 0 1] Processed Events
  ;[1 0.008092 0] Play Multiple Audio
  (Utilities|FlowControl|Sequence
    (:then_0
      (bind (_array_element _array_index) (Utilities|Array|ForEachLoopwithBreak _2d_sound_items :!label _label)
        (:LoopBody
          (if (and (== (.Track (Utilities|Struct|BreakFWaveTracker _array_element)) track) (== (.Note (Utilities|Struct|BreakFWaveTracker _array_element)) note))
            (Audio|Components|Audio|Stop (.Audio (Utilities|Struct|BreakFWaveTracker _array_element)))
            (Utilities|Array|RemoveIndex _2d_sound_items _array_index)
            (goto _label Break)))))
    (:then_1
      (if (!= velocity 0)
        (bind _returnvalue (Class|SoundUtils|ConstantNote 2048.0 (Class|MidiUtils|NotetoFrequency note)))
        (bind _returnvalue_2 (Audio|SpawnSound2D _returnvalue 1.0 1.0))
        (Utilities|Array|Add (Variables|Default|Get2D%20Sound%20Items) (Utilities|Struct|MakeFWaveTracker track note _returnvalue_2))))))

(event EventBeginPlay
  ;[0 1 0.6045] Setup Midi
  (|CallParentFunction))

(fn ConstructionScript)