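; MIDI player actor that plays the level's MIDI asset to a MIDI output and drives a music visualizer stage.
; BeginPlay spawns the keyboard, statues, dust, ball and beat-linked floating objects.
; Note events, filtered by separate play and visualize channel lists, drive keyboard, ball, statue colors and electricity arcs, with channel 8 also triggering one-time rain.
; Tempo PPQ sets the tick threshold that fires Beat events.
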(event OnEventTempo(Midi)
  (params (mpqn :type Integer) (ppq :type Integer))
  ;[1 1 1] Tempo Event
  (bind _output_get (Variables|Midi|SetMidiMPQN mpqn))
  (bind _output_get_2 (Variables|Midi|SetMidiPPQ ppq))
  (CallFunction|SetBeatTicksTreshold _output_get_2)
  (Development|PrintString (Utilities|String|Append "New MPQN " (Utilities|String|ToString(Integer) _output_get) "| PPQ " (Utilities|String|ToString(Integer) _output_get_2)) true true "(R=0.000000,G=0.660000,B=1.000000,A=1.000000)" 1e+01))

(event OnSend(Midi)
  (params (msg :type Array%20of%20Bytes) (elapsed :type Integer) (channel :type Integer) (midiEventType :type Integer))
  ;[1 1 1] Device Midi Synth
  (bind _playnote (CallFunction|ShouldNotebePlayed channel midiEventType))
  (if _playnote
    (Class|MidiInterface|SendMidiMessage msg)))

(event OnEventTicks(Midi)
  (params (ticksElapsed :type Integer))
  ;[1 1 1] Ticks Event
  (if (< ticksElapsed (Variables|Default|GetLastTicksElapsed))
    (Variables|Midi|SetTicksElapsed (- (Variables|Midi|GetTicksElapsed) (Variables|Default|GetLastTicksElapsed)))
    (Variables|Default|SetLastTicksElapsed 0))
  (if (> (- ticksElapsed (Variables|Default|GetLastTicksElapsed)) (Variables|Default|GetTicksForBeatStepTreshold))
    (bind _output_get (Variables|Default|SetLastTicksElapsed (+ (Variables|Default|GetLastTicksElapsed) (Variables|Default|GetTicksForBeatStep))))
    (Development|PrintString (Utilities|String|ToString(Integer) _output_get))
    (Variables|Default|SetLastTicksElapsed (+ (Variables|Default|GetLastTicksElapsed) (Variables|Default|GetTicksForBeatStep)))
    (Class|BeatComponent|CallBeatEvent (Variables|Default|GetBeat))))

(event OnEventwithInfo(Midi)
  (params (track :type Integer) (note :type Integer) (velocity :type Integer) (nextNote :type Integer) (timeDifference :type Integer) (eventType :type Integer) (elapsed :type Integer))
  (bind _visualstatues (Variables|Default|GetVisualStatues))
  ;[1 1 1] Processing Visual Events
  ;;[0.1203 0 1] Processed Events
  (bind _playnote (CallFunction|ShouldNotebeVisualized track eventType))
  (if _playnote
    (Variables|Midi|SetCurrentNoteVelocity velocity)
    (Variables|Midi|SetCurrentNote note)
    (Variables|Midi|SetChannel track)
    (Variables|Midi|SetNextNote nextNote)
    (Variables|Midi|SetTimeDifference timeDifference)
    (Variables|Midi|SetMidiEventType eventType)
    (if (and (== (Variables|Midi|GetChannel) 0) (== (Variables|Midi|GetMidiEventType) (Variables|Midi|GetMidiNoteOn)))
      (Default|UpdatePosition (Variables|Default|GetBall) (Variables|Midi|GetNextNote) (Variables|Midi|GetTimeDifference)))
    (Default|Update (Variables|Default|GetMidiKeyboard) (Variables|Midi|GetChannel) (Variables|Midi|GetCurrentNote) (Variables|Midi|GetNextNote) (Variables|Midi|GetTimeDifference) (Variables|Midi|GetMidiEventType))
    (if (== (Variables|Midi|GetChannel) 8)
      (if (!= (Variables|Midi|GetCurrentNoteVelocity) 0)
        (if (Variables|Default|GetbRainSpawned)
          _
          (else
            (CallFunction|SpawnRain)
            (Variables|Default|SetbRainSpawned true)))
        (bind _newparam (CallFunction|SpawnEmitter (Variables|Midi|GetCurrentNote)))
        (Variables|Default|SetEmitter _newparam)
        (else
          (Utilities|IsValid (Variables|Default|GetEmitter)
            (:Is%20Valid
              (Actor|DestroyActor (Variables|Default|GetEmitter))))))
      (elif (== (Variables|Midi|GetChannel) 4)
        (Rendering|Material|SetVectorParameterValue (Utilities|Array|Get(acopy) _visualstatues) "Color" (Math|Color|SelectColor (Utilities|Array|Get(acopy) (Variables|Default|GetVisualCubesColors) (Variables|Midi|GetChannel)) "(R=0.000000,G=0.000000,B=0.000000,A=1.000000)" (!= (Variables|Midi|GetCurrentNoteVelocity) 0)) :!class /Script/Engine.MaterialInstanceDynamic)
        (Rendering|Material|SetVectorParameterValue (Utilities|Array|Get(acopy) _visualstatues 1) "Color" (Math|Color|SelectColor (Utilities|Array|Get(acopy) (Variables|Default|GetVisualCubesColors) (Variables|Midi|GetChannel)) "(R=0.000000,G=0.000000,B=0.000000,A=1.000000)" (!= (Variables|Midi|GetCurrentNoteVelocity) 0)) :!class /Script/Engine.MaterialInstanceDynamic)))))

(event OnEvent(Midi)
  (params (track :type Integer) (note :type Integer) (velocity :type Integer) (elapsed :type Integer)))

(event Custom|PlayTrack
  (bind _midi (Variables|Default|GetMidi))
  ;[1 1 1] Play Track
  (Class|MidiComponent|LoadAsset _midi (Variables|Default|GetMidi%20Asset))
  (Class|MidiComponent|Start _midi)
  (Default|CallOnChangeSunPosition 0.0))

(event Custom|PlayTrackLooped
  (bind _midi (Variables|Default|GetMidi))
  (Class|MidiComponent|LoadAsset _midi (Variables|Default|GetMidi%20Asset))
  (Class|MidiComponent|StartwithLoop _midi 1 2))

(event Custom|MidiStopped
  (params (finished :type Boolean))
  ;[1 1 1] Device Midi Synth
  (Development|PrintString "Stop")
  (CallFunction|StopVizualize))

(event Custom|StopTrack
  ;[1 1 1] Stop Track
  (Class|MidiComponent|Stop (Variables|Default|GetMidi))
  (CallFunction|StopVizualize)
  (Default|CallOnChangeSunPosition -5.0))

(event Custom|ChangeLoopRange
  (params (StartBar :type Integer) (EndBar :type Integer))
  (Class|MidiComponent|SetLoopRange (Variables|Default|GetMidi) StartBar EndBar))

(event EventEndPlay
  (params (EndPlayReason :type EEndPlayReason%20Enum :default "Destroyed"))
  ;[1 1 1] Device Midi Synth
  (Class|MidiInterface|CloseMidiOutput)
  (CallFunction|StopVizualize))

(event EventBeginPlay
  ;[0 1 0.6045] Setup Midi
  (|CallParentFunction)
  (EventDispatchers|BindEventtoOnStop (Variables|Default|GetMidi) (delegate Custom|MidiStopped))
  ;[1 1 1] Create Visual Cubes
  (Utilities|FlowControl|Sequence
    (:then_0
      (bind _asmy_game_instance (Utilities|Casting|CastToMyGameInstance (Game|GetGameInstance (Game|Player|GetPlayerPawn 0))))
      (Variables|Default|SetMidi%20Asset (Variables|/Game/GameInstances/MyGameInstance.MyGameInstance_C|GetLevelMidiAsset _asmy_game_instance)))
    (:then_1
      (bind _returnvalue (Game|SpawnActorfromClass "/Game/Blueprints/VisualBoxes.VisualBoxes_C" (Math|Transform|MakeTransform "0,-287.000000,60.000000" "0, 0, 0" "1,1,1") "Undefined" 0 0))
      (Variables|Default|SetMidiKeyboard _returnvalue)
      (for _index (range 0 20)
        (Utilities|Array|Add (Variables|Default|GetVisualCubesColors) (Utilities|Struct|MakeLinearColor (Math|Random|RandomFloat) (Math|Random|RandomFloat) (Math|Random|RandomFloat) 1.0)))
      (bind _returnvalue_2 (Game|SpawnActorfromClass "/Game/Statue_BP.Statue_BP_C" (Math|Transform|MakeTransform (Math|Vector|MakeVector -25.0 8e+02 3e+01) "0, 0, 0" "1,1,1") "AdjustIfPossibleButAlwaysSpawn" 0 0))
      (bind _returnvalue_3 (Rendering|Material|CreateDynamicMaterialInstance (Variables|/Game/Statue_BP.Statue_BP_C|GetStaticMesh _returnvalue_2) 0 "/Game/Materials/MatTest.MatTest" :!class /Script/Engine.PrimitiveComponent))
      (Utilities|Array|Add (Variables|Default|GetVisualStatues) _returnvalue_3)
      (bind _returnvalue_4 (Game|SpawnActorfromClass "/Game/Statue_BP.Statue_BP_C" (Math|Transform|MakeTransform (Math|Vector|MakeVector -25.0 -8e+02 3e+01) "0, 0, 0" "1,1,1") "AdjustIfPossibleButAlwaysSpawn" 0 0))
      (bind _returnvalue_5 (Rendering|Material|CreateDynamicMaterialInstance (Variables|/Game/Statue_BP.Statue_BP_C|GetStaticMesh _returnvalue_4) 0 "/Game/Materials/MatTest.MatTest" :!class /Script/Engine.PrimitiveComponent))
      (Utilities|Array|Add (Variables|Default|GetVisualStatues) _returnvalue_5)
      (bind _returnvalue_6 (Game|SpawnActorfromClass "/Game/Blueprints/DustDrops.DustDrops_C" (Math|Transform|MakeTransform (Math|Vector|MakeVector -1e+03 -2e+02 4e+02) "-40.000000,25.000000, 0" "1,1,1") "Undefined" 0 0))
      (Variables|Default|SetDust _returnvalue_6)
      (bind _returnvalue_7 (Game|SpawnActorfromClass "/Game/Blueprints/Midi_Ball.Midi_Ball_C" (Math|Transform|MakeTransform (+ (Variables|Default|GetStartLocation) "0, 0,220.000000") "0, 0, 0" "1,1,1") "Undefined" 0 0))
      (Variables|Default|SetBall _returnvalue_7)
      (CallFunction|SpawnFloatingObjects (Variables|Default|GetFloatingObjectsAmount)))))

(fn ConstructionScript)

(fn SpawnEmitter
  (params (Note :type Integer))
  (bind _emitter (Variables|Default|GetEmitter))
  (Utilities|IsValid _emitter
    (:Is%20Valid
      (Actor|DestroyActor _emitter))
    (:Is%20Not%20Valid
      _))
  (LocalVariables|SetHeight (+ (* (Math|Conversions|ToFloat(Integer) Note) 7.0) 8e+01))
  (bind _returnvalue (Game|SpawnActorfromClass "/Game/ElectricityArc_BP.ElectricityArc_BP_C" (Math|Transform|MakeTransform (Math|Vector|MakeVector 0.0 -6.5e+02 (LocalVariables|GetHeight)) "0, 0, 0" "1,1,1") "AlwaysSpawn" 0 0))
  (Class|ParticleSystemComponent|SetBeamTargetPoint (Variables|/Game/ElectricityArc_BP.ElectricityArc_BP_C|GetEmitter _returnvalue) 0 (Math|Vector|MakeVector 0.0 6.5e+02 (LocalVariables|GetHeight)))
  (return _returnvalue))

(fn SpawnRain
  (for _index (range 0 3)
    (Game|SpawnActorfromClass "/Game/Blueprints/WaterDrops.WaterDrops_C" (Math|Transform|MakeTransform (Math|Vector|MakeVector -5e+02 (+ (* _index 3e+02) -6e+02) 8e+02) "0, 0, 0" "1,1,1") "Undefined" 0 0))
  (Actor|DestroyActor (Variables|Default|GetDust)))

(fn ShouldNotebePlayed
  (params (ChannelNumber :type Integer) (EventType :type Integer))
  (return (or (Utilities|Array|ContainsItem (Variables|Midi|GetChannelsToPlay) ChannelNumber) (== EventType (LocalVariables|GetNoteOffEventType)))))

(fn AddChanneltoPlay
  (params (ChannelToAdd :type Integer))
  (Utilities|Array|AddUnique (Variables|Midi|GetChannelsToPlay) ChannelToAdd)
  (CallFunction|AddChanneltoVisualize ChannelToAdd))

(fn RemoveChanneltoPlay
  (params (RemoveChannel :type Integer))
  (Utilities|Array|RemoveItem (Variables|Midi|GetChannelsToPlay) RemoveChannel)
  (CallFunction|RemoveChanneltoVisualize RemoveChannel))

(fn SwitchChanneltoPlay
  (params (Channel :type Integer))
  (if (Utilities|Array|ContainsItem (Variables|Midi|GetChannelsToPlay) Channel)
    (CallFunction|RemoveChanneltoPlay Channel)
    (else
      (CallFunction|AddChanneltoPlay Channel))))

(fn ShouldNotebeVisualized
  (params (Channel :type Integer) (EventType :type Integer))
  (return (or (Utilities|Array|ContainsItem (Variables|Midi|GetChannelsToVisualize) Channel) (== EventType (LocalVariables|GetNoteOffEventType)))))

(fn AddChanneltoVisualize
  (params (Channel :type Integer))
  (Utilities|Array|AddUnique (Variables|Midi|GetChannelsToVisualize) Channel))

(fn RemoveChanneltoVisualize
  (params (Channel :type Integer))
  (Utilities|Array|RemoveItem (Variables|Midi|GetChannelsToVisualize) Channel))

(fn SpawnFloatingObjects
  (params (Amount :type Integer))
  (bind _outactors (Actor|GetAllActorsOfClass "/Game/Blueprints/Floating_SpawnArea.Floating_SpawnArea_C"))
  (for _array_element _outactors
    (Utilities|IsValid _array_element
      (:Is%20Valid
        (for _index (range 1 Amount)
          (bind _position (Default|GetNewSpawnPosition3D _array_element 0 "/Game/Blueprints/SIO_Floating.SIO_Floating_C"))
          (Game|SpawnActorfromClass "/Game/Blueprints/SIO_Floating.SIO_Floating_C" (Math|Transform|MakeTransform (Transformation|GetActorLocation _array_element) "90.000000, 0, 0" "1,1,1") "Undefined" 0 _position 25 (Variables|Default|GetBeat)))))))

(fn SetBeatTicksTreshold
  (params (PPQ :type Integer))
  (Variables|Default|SetTicksForBeatStep PPQ)
  (bind _output_get (Variables|Default|SetTicksForBeatStepTreshold (Math|Float|Truncate (* (Variables|Default|GetTicksForBeatStep) 2.05))))
  (Development|PrintString (Utilities|String|ToString(Integer) _output_get)))

(fn StopVizualize
  (Default|TurnOffAll (Variables|Default|GetMidiKeyboard))
  (Variables|Midi|SetTicksElapsed 0)
  (Variables|Default|SetLastTicksElapsed 0))