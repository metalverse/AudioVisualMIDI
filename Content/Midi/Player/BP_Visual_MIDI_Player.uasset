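; Actor that visualizes MIDI playback as a row of cubes, one per note number, lit in the color of the track playing it.
; BeginPlay spawns the static mesh components along Y, gives each a dynamic material instance and generates a random color palette for tracks.
; Midi's OnEvent indexes the material by note and sets its Color parameter to the track's color, or black when velocity is zero.
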(event OnEvent(Midi)
  (params (track :type Integer) (note :type Integer) (velocity :type Integer) (elapsed :type Integer))
  ;[0.1203 0 1] Processed Events
  (Rendering|Material|SetVectorParameterValue (Utilities|Array|Get(acopy) (Variables|Default|GetVisual%20Cubes) note) "Color" (Math|Color|SelectColor (Utilities|Array|Get(acopy) (Variables|Default|GetVisualCubesColors) track) "(R=0.000000,G=0.000000,B=0.000000,A=1.000000)" (!= velocity 0)) :!class /Script/Engine.MaterialInstanceDynamic))

(event EventBeginPlay
  ;[0 1 0.6045] Setup Midi
  (|CallParentFunction)
  ;[1 1 1] Create Visual Cubes
  (for _index (range 0 120)
    (bind _returnvalue (AddComponent|AddStaticMeshComponent false (Math|Transform|MakeTransform (Math|Vector|MakeVector 0.0 (* _index 1e+02) 0.0) "0, 0, 0" "0.500000,0.500000,0.500000")))
    (bind _returnvalue_2 (Rendering|Material|CreateDynamicMaterialInstance _returnvalue 0 "/Game/Materials/MatTest.MatTest" :!class /Script/Engine.PrimitiveComponent))
    (Utilities|Array|Add (Variables|Default|GetVisual%20Cubes) _returnvalue_2))
  (for _index_2 (range 0 20)
    (Utilities|Array|Add (Variables|Default|GetVisualCubesColors) (Utilities|Struct|MakeLinearColor (Math|Random|RandomFloat) (Math|Random|RandomFloat) (Math|Random|RandomFloat) 1.0))))

(fn ConstructionScript)