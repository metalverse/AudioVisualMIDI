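; Actor that visualizes MIDI playback as a row of colored cubes.
; On BeginPlay it creates 16 half-scale mesh components along Y, each with its own dynamic material instance stored in an array.
; Midi events use the track number as the array index, setting that material's Color to a random color for nonzero velocity, or black for zero velocity.
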(event OnEvent(Midi)
  (params (track :type Integer) (note :type Integer) (velocity :type Integer) (elapsed :type Integer))
  ;[0.1203 0 1] Processed Events
  ;[1 1 1] Visualization Cube
  (Rendering|Material|SetVectorParameterValue (Utilities|Array|Get(acopy) (Variables|Default|GetVisual%20Cubes) track) "Color" (Math|Color|SelectColor :A (Math|Color|MakeColor (Math|Random|RandomFloat) (Math|Random|RandomFloat) (Math|Random|RandomFloat) 0.0) :bPickA (!= 0 velocity)) :!class /Script/Engine.MaterialInstanceDynamic))

(event EventBeginPlay
  ;[0 1 0.6045] Setup Midi
  (|CallParentFunction)
  ;[1 1 1] Create Visual Cubes
  (for _index (range 0 15)
    (bind _returnvalue (AddComponent|AddStaticMeshComponent false (Math|Transform|MakeTransform (Math|Vector|MakeVector 0.0 (* _index 1e+02) 0.0) "0.000000, 0, 0" "0.500000,0.500000,0.500000")))
    (bind _returnvalue_2 (Rendering|Material|CreateDynamicMaterialInstance _returnvalue 0 "/Game/Midi/Other/MatTest.MatTest" :!class /Script/Engine.PrimitiveComponent))
    (Utilities|Array|Add (Variables|Default|GetVisual%20Cubes) _returnvalue_2)))

(fn ConstructionScript)