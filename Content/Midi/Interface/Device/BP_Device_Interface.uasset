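; Blueprint that interfaces with a MIDI device through a MidiInterface.
; BeginPlay opens input device 0 and prints an on-screen error if that fails, while EndPlay calls CloseMidiOutput rather than closing the input.
; The receive event is an empty stub.
; CheckOnOffEvent bit-masks the first byte to detect note on/off, though its 128 test matches any byte with the high bit set.
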(event OnReceive(MidiInterface)
  (params (msg :type Array%20of%20Bytes) (deltaTime :type Float%20%28single-precision%29))
  ;[1 1 1] When Event Is Received
)

(event EventBeginPlay
  ;[1 1 1] Midi Device Interfacing
  (bind _returnvalue (Class|MidiInterfaceComponent|OpenInput (Variables|Default|GetMidiInterface)))
  (if (not _returnvalue)
    (Development|PrintString "Unable to run Blueprint (Missing Input Device)" true false "(R=1.000000,G=0.100000,B=0.100000,A=1.000000)" 4.0)))

(event EventEndPlay
  (params (EndPlayReason :type EEndPlayReason%20Enum :default "Destroyed"))
  ;[1 1 1] Midi Device Interfacing
  (Class|MidiInterface|CloseMidiOutput))

(fn ConstructionScript)

(fn CheckOn/OffEvent
  (params (TargetArray :type Array%20of%20Bytes))
  (bind _item (Utilities|Array|Get(acopy) TargetArray))
  (bind _returnvalue (Math|Conversions|ToInteger(Byte) _item))
  (return (or (== 128 (Class|KismetMathLibrary|AndIntInt 128 _returnvalue)) (== 144 (Class|KismetMathLibrary|AndIntInt 144 _returnvalue)))))