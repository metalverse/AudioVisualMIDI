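; MIDI input interface Blueprint that plays incoming notes as generated 2D tones, with device setup on BeginPlay.
; Received messages that pass an on/off check first stop and remove any tracked sound with the same note on track 0.
; A second check gates spawning a constant-note sound at the note's frequency.
; Each sound is stored with its track and note, allowing several notes to play at once.
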(event OnReceive(MidiInterface)
  (params (msg :type Array%20of%20Bytes) (deltaTime :type Float%20%28single-precision%29))
  (bind _item (Utilities|Array|Get(acopy) msg 1))
  (bind _returnvalue (Class|KismetSystemLibrary|MakeLiteralInteger))
  (bind _newparam (CallFunction|CheckOn/OffEvent msg))
  (bind _2d_sound_items (Variables|Default|Get2D%20Sound%20Items))
  (bind _returnvalue_2 (Math|Conversions|ToInteger(Byte) _item))
  ;[0.1203 0 1] Processed Input Events
  (if _newparam
    ;[1 0.008092 0] Play Multiple Audio
    (Utilities|FlowControl|Sequence
      (:then_0
        (bind (_array_element _array_index) (Utilities|Array|ForEachLoopwithBreak _2d_sound_items :!label _label)
          (:LoopBody
            (if (and (== (.Track (Utilities|Struct|BreakFWaveTracker _array_element)) _returnvalue) (== (.Note (Utilities|Struct|BreakFWaveTracker _array_element)) _returnvalue_2))
              (Audio|Components|Audio|Stop (.Audio (Utilities|Struct|BreakFWaveTracker _array_element)))
              (Utilities|Array|RemoveIndex _2d_sound_items _array_index)
              (goto _label Break)))))
      (:then_1
        (if _newparam
          (bind _returnvalue_3 (Class|SoundUtils|ConstantNote 2048.0 (Class|MidiUtils|NotetoFrequency _returnvalue_2)))
          (bind _returnvalue_4 (Audio|SpawnSound2D _returnvalue_3 1.0 1.0))
          (Utilities|Array|Add (Variables|Default|Get2D%20Sound%20Items) (Utilities|Struct|MakeFWaveTracker _returnvalue _returnvalue_2 _returnvalue_4)))))))

(event EventBeginPlay
  ;[0 1 0.6045] Setup Midi Input Device
  (|CallParentFunction))

(fn ConstructionScript)