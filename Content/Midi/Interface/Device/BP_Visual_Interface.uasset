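; BP_Visual_Interface is a MIDI device Blueprint that visualizes received note on/off events as a row of colored cubes.
; BeginPlay opens MIDI output 0 and spawns 128 small static mesh components, storing a dynamic material instance for each.
; On receive, on/off messages use the note byte to pick a material, toggling it between random color and black.
; Note state is inferred by toggling membership in the INDEX array.
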(event OnReceive(MidiInterface)
  (params (msg :type Array%20of%20Bytes) (deltaTime :type Float%20%28single-precision%29))
  (bind _item (Utilities|Array|Get(acopy) msg 1))
  (bind _index (Variables|Default|GetINDEX))
  (if (CallFunction|CheckOn/OffEvent msg)
    ;[1 1 1] Visualization Cube
    (Rendering|Material|SetVectorParameterValue (Utilities|Array|Get(acopy) (Variables|Default|GetVisual%20Cubes) (Math|Conversions|ToInteger(Byte) _item)) "Color" (Math|Color|SelectColor :A (Math|Color|MakeColor (Math|Random|RandomFloat) (Math|Random|RandomFloat) (Math|Random|RandomFloat) 0.0) :bPickA (not (Utilities|Array|ContainsItem (Variables|Default|GetINDEX) _item))) :!class /Script/Engine.MaterialInstanceDynamic)
    ;[1 1 1] Messy Check Array of On/Off Events
    (if (Utilities|Array|ContainsItem _index _item)
      (Utilities|Array|RemoveItem _index _item)
      (else
        (Utilities|Array|Add _index _item)))))

(event EventBeginPlay
  ;[1 1 1] Midi Device Interfacing
  (|CallParentFunction)
  (Class|MidiInterface|OpenMidiOutput)
  ;[1 1 1] Create Visual Cubes
  (for _index (range 0 127)
    (bind _returnvalue (AddComponent|AddStaticMeshComponent false (Math|Transform|MakeTransform (Math|Vector|MakeVector 0.0 (* _index 2e+01) 0.0) "0, 0, 0" "0.100000,0.100000,0.100000")))
    (bind _returnvalue_2 (Rendering|Material|CreateDynamicMaterialInstance _returnvalue 0 "/Game/Materials/MatTest.MatTest" :!class /Script/Engine.PrimitiveComponent))
    (Utilities|Array|Add (Variables|Default|GetVisual%20Cubes) _returnvalue_2)))

(fn ConstructionScript)