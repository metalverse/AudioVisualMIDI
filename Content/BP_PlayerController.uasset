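; Player controller that switches the channel of a visual MIDI player from the keyboard.
; On BeginPlay it finds BP_Visual_MIDI_Player_Plus actors in the level and caches the first valid one.
; The 0, 1 and 2 keys call SwitchChannel on that cached player with the matching channel index.
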(event EventBeginPlay
  (bind _outactors (Actor|GetAllActorsOfClass "/Game/Midi/Player/BP_Visual_MIDI_Player_Plus.BP_Visual_MIDI_Player_Plus_C"))
  (Utilities|IsValid (Utilities|Array|Get(acopy) _outactors)
    (:Is%20Valid
      (Variables|Default|SetMidiVisualPlayer (Utilities|Array|Get(acopy) _outactors)))))

(event EventTick
  (params (DeltaSeconds :type Float%20%28single-precision%29)))

(event Input|KeyboardEvents|1
  (params (Key :type Key%20Structure :default "AnyKey"))
  (bind _midivisualplayer (Variables|Default|GetMidiVisualPlayer))
  (:Pressed
    (Utilities|IsValid _midivisualplayer
      (:Is%20Valid
        (Default|SwitchChannel _midivisualplayer 1)))))

(event Input|KeyboardEvents|2
  (params (Key :type Key%20Structure :default "AnyKey"))
  (bind _midivisualplayer (Variables|Default|GetMidiVisualPlayer))
  (:Pressed
    (Utilities|IsValid _midivisualplayer
      (:Is%20Valid
        (Default|SwitchChannel _midivisualplayer 2)))))

(event Input|KeyboardEvents|0
  (params (Key :type Key%20Structure :default "AnyKey"))
  (bind _midivisualplayer (Variables|Default|GetMidiVisualPlayer))
  (:Pressed
    (Utilities|IsValid _midivisualplayer
      (:Is%20Valid
        (Default|SwitchChannel _midivisualplayer)))))

(fn ConstructionScript)